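; Spotlight mover that drives the lights of BP_Spotlights from a dancer's body motion.
; Each Tick caches limb velocities and rotations through the dancer interface, found via BP_Spotlights.
; With body control on, velocities set intensities and rotations steer balls and hinges with VInterpTo smoothing.
; Head control hands the higher lights to the head; EndSequence fades the intensity range to zero by timeline, and Restart resets it.
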(event EventTick
  (params (DeltaSeconds :type Float%20%28single-precision%29))
  (Variables|Default|SetDelta%20Seconds DeltaSeconds)
  (Utilities|FlowControl|Sequence
    (:then_0
      (if (Variables|Default|GetDancerFound)
        (bind _velocity (Default|GetLForeArmVelocity (Variables|Default|GetBPI_Dancer)))
        (Utilities|Array|SetArrayElem (Variables|Default|GetVelocities) 0 (Math|Vector|MakeVector (Math|Float|Absolute(Float) (.x _velocity)) (Math|Float|Absolute(Float) (.y _velocity)) (Math|Float|Absolute(Float) (.z _velocity))) true)
        (bind _velocity_2 (Default|GetLHandVelocity (Variables|Default|GetBPI_Dancer)))
        (Utilities|Array|SetArrayElem (Variables|Default|GetVelocities) 1 (Math|Vector|MakeVector (Math|Float|Absolute(Float) (.x _velocity_2)) (Math|Float|Absolute(Float) (.y _velocity_2)) (Math|Float|Absolute(Float) (.z _velocity_2))) true)
        (bind _velocity_3 (Default|GetLLegVelocity (Variables|Default|GetBPI_Dancer)))
        (Utilities|Array|SetArrayElem (Variables|Default|GetVelocities) 2 (Math|Vector|MakeVector (Math|Float|Absolute(Float) (.x _velocity_3)) (Math|Float|Absolute(Float) (.y _velocity_3)) (Math|Float|Absolute(Float) (.z _velocity_3))) true)
        (bind _velocity_4 (Default|GetLToeVelocity (Variables|Default|GetBPI_Dancer)))
        (Utilities|Array|SetArrayElem (Variables|Default|GetVelocities) 3 (Math|Vector|MakeVector (Math|Float|Absolute(Float) (.x _velocity_4)) (Math|Float|Absolute(Float) (.y _velocity_4)) (Math|Float|Absolute(Float) (.z _velocity_4))) true)
        (bind _velocity_5 (Default|GetRForeArmVelocity (Variables|Default|GetBPI_Dancer)))
        (Utilities|Array|SetArrayElem (Variables|Default|GetVelocities) 4 (Math|Vector|MakeVector (Math|Float|Absolute(Float) (.x _velocity_5)) (Math|Float|Absolute(Float) (.y _velocity_5)) (Math|Float|Absolute(Float) (.z _velocity_5))) true)
        (bind _velocity_6 (Default|GetRHandVelocity (Variables|Default|GetBPI_Dancer)))
        (Utilities|Array|SetArrayElem (Variables|Default|GetVelocities) 5 (Math|Vector|MakeVector (Math|Float|Absolute(Float) (.x _velocity_6)) (Math|Float|Absolute(Float) (.y _velocity_6)) (Math|Float|Absolute(Float) (.z _velocity_6))) true)
        (bind _velocity_7 (Default|GetRLegVelocity (Variables|Default|GetBPI_Dancer)))
        (Utilities|Array|SetArrayElem (Variables|Default|GetVelocities) 6 (Math|Vector|MakeVector (Math|Float|Absolute(Float) (.x _velocity_7)) (Math|Float|Absolute(Float) (.y _velocity_7)) (Math|Float|Absolute(Float) (.z _velocity_7))) true)
        (bind _velocity_8 (Default|GetRToeVelocity (Variables|Default|GetBPI_Dancer)))
        (Utilities|Array|SetArrayElem (Variables|Default|GetVelocities) 7 (Math|Vector|MakeVector (Math|Float|Absolute(Float) (.x _velocity_8)) (Math|Float|Absolute(Float) (.y _velocity_8)) (Math|Float|Absolute(Float) (.z _velocity_8))) true)
        (bind _transform (Default|GetLForeArmTransform (Variables|Default|GetBPI_Dancer)))
        (Utilities|Array|SetArrayElem (Variables|Default|GetTransform%20Rotation) 0 (.rotation _transform) true)
        (bind _transform_2 (Default|GetLHandTransform (Variables|Default|GetBPI_Dancer)))
        (Utilities|Array|SetArrayElem (Variables|Default|GetTransform%20Rotation) 1 (.rotation _transform_2) true)
        (bind _transform_3 (Default|GetLLegTransform (Variables|Default|GetBPI_Dancer)))
        (Utilities|Array|SetArrayElem (Variables|Default|GetTransform%20Rotation) 2 (.rotation _transform_3) true)
        (bind _transform_4 (Default|GetLToeTransform (Variables|Default|GetBPI_Dancer)))
        (Utilities|Array|SetArrayElem (Variables|Default|GetTransform%20Rotation) 3 (.rotation _transform_4) true)
        (bind _transform_5 (Default|GetRForeArmTransform (Variables|Default|GetBPI_Dancer)))
        (Utilities|Array|SetArrayElem (Variables|Default|GetTransform%20Rotation) 4 (.rotation _transform_5) true)
        (bind _transform_6 (Default|GetRHandTransform (Variables|Default|GetBPI_Dancer)))
        (Utilities|Array|SetArrayElem (Variables|Default|GetTransform%20Rotation) 5 (.rotation _transform_6) true)
        (bind _transform_7 (Default|GetRLegTransform (Variables|Default|GetBPI_Dancer)))
        (Utilities|Array|SetArrayElem (Variables|Default|GetTransform%20Rotation) 6 (.rotation _transform_7) true)
        (bind _transform_8 (Default|GetRToeTransform (Variables|Default|GetBPI_Dancer)))
        (Utilities|Array|SetArrayElem (Variables|Default|GetTransform%20Rotation) 7 (.rotation _transform_8) true)
        (else
          (bind _returnvalue (Actor|GetActorOfClass "/PremierLaserShow/Blueprints/BP_Spotlights.BP_Spotlights_C"))
          (bind _output_get (Variables|Default|SetBPI_Dancer (Variables|/PremierLaserShow/Blueprints/BP_Spotlights.BP_Spotlights_C|GetDancerSkeleton _returnvalue)))
          (Utilities|IsValid (Utilities|ToObject(Interface) _output_get)
            (:Is%20Valid
              (Variables|Default|SetDancerFound true))))))
    (:then_1
      (if (Variables|Default|GetStartBodyControl)
        (bind _returnvalue_2 (Actor|GetActorOfClass "/PremierLaserShow/Blueprints/BP_Spotlights.BP_Spotlights_C"))
        (Variables|/PremierLaserShow/Blueprints/BP_Spotlights.BP_Spotlights_C|SetCircumventOrder _returnvalue_2 true)
        (Utilities|FlowControl|Sequence
          (:then_0
            (for (_array_element _array_index) (Variables|/PremierLaserShow/Blueprints/BP_Spotlights.BP_Spotlights_C|GetSpotlightsLower _returnvalue_2)
              (Rendering|Components|Light|SetIntensity _array_element (Math|Float|Lerp (Variables|Default|GetIntensityMin) (Variables|Default|GetIntensityMax) (Math|Float|Absolute(Float) (.z (Utilities|Array|Get(acopy) (Variables|Default|GetVelocities) _array_index)))))))
          (:then_1
            (for (_array_element_2 _array_index_2) (Variables|/PremierLaserShow/Blueprints/BP_Spotlights.BP_Spotlights_C|GetSpotlightBallsLower _returnvalue_2)
              (Transformation|SetRelativeRotation _array_element_2 (Math|Rotator|MakeRotator (.roll (.rotation (Transformation|GetRelativeTransform _array_element_2))) (.pitch (.rotation (Transformation|GetRelativeTransform _array_element_2))) (.z (Math|Interpolation|VInterpTo (Math|Vector|MakeVector 0.0 0.0 (.yaw (.rotation (Transformation|GetRelativeTransform _array_element_2)))) (Math|Vector|MakeVector 0.0 0.0 (.yaw (Utilities|Array|Get(acopy) (Variables|Default|GetTransform%20Rotation) _array_index_2))) (Variables|Default|GetDelta%20Seconds) 1.0))) false false)))
          (:then_2
            (for (_array_element_3 _array_index_3) (Variables|/PremierLaserShow/Blueprints/BP_Spotlights.BP_Spotlights_C|GetSpotlightHingesLower _returnvalue_2)
              (Transformation|SetRelativeRotation _array_element_3 (Math|Rotator|MakeRotator (.x (Math|Interpolation|VInterpTo (Math|Vector|MakeVector (.roll (.rotation (Transformation|GetRelativeTransform _array_element_3))) 0.0 0.0) (Math|Vector|MakeVector (.pitch (Utilities|Array|Get(acopy) (Variables|Default|GetTransform%20Rotation) _array_index_3)) 0.0 0.0) (Variables|Default|GetDelta%20Seconds) 1.0)) (.pitch (.rotation (Transformation|GetRelativeTransform _array_element_3))) (.yaw (.rotation (Transformation|GetRelativeTransform _array_element_3)))) false false)))
          (:then_3
            (if (Variables|Default|GetStartHeadControl)
              (for _array_element_4 (Variables|/PremierLaserShow/Blueprints/BP_Spotlights.BP_Spotlights_C|GetSpotlightsHigher _returnvalue_2)
                (bind _velocity_9 (Default|GetHeadVelocity (Variables|Default|GetBPI_Dancer)))
                (Rendering|Components|Light|SetIntensity _array_element_4 (Math|Float|Lerp (Variables|Default|GetIntensityMin) (Variables|Default|GetIntensityMax) (Math|Float|Absolute(Float) (.x _velocity_9)))))
              (else
                (for (_array_element_5 _array_index_4) (Variables|/PremierLaserShow/Blueprints/BP_Spotlights.BP_Spotlights_C|GetSpotlightsHigher _returnvalue_2)
                  (Rendering|Components|Light|SetIntensity _array_element_5 (Math|Float|Lerp (Variables|Default|GetIntensityMin) (Variables|Default|GetIntensityMax) (Math|Float|Absolute(Float) (.y (Utilities|Array|Get(acopy) (Variables|Default|GetVelocities) _array_index_4)))))))))
          (:then_4
            (if (Variables|Default|GetStartHeadControl)
              (for _array_element_6 (Variables|/PremierLaserShow/Blueprints/BP_Spotlights.BP_Spotlights_C|GetSpotlightHingesHigher _returnvalue_2)
                (bind _transform_9 (Default|GetHeadTransform (Variables|Default|GetBPI_Dancer)))
                (Transformation|SetRelativeRotation _array_element_6 (Math|Rotator|MakeRotator (.roll (.rotation (Transformation|GetRelativeTransform _array_element_6))) (.pitch (.rotation (Transformation|GetRelativeTransform _array_element_6))) (.z (Math|Interpolation|VInterpTo (Math|Vector|MakeVector 0.0 0.0 (.yaw (.rotation (Transformation|GetRelativeTransform _array_element_6)))) (Math|Vector|MakeVector 0.0 0.0 (.yaw (.rotation _transform_9))) (Variables|Default|GetDelta%20Seconds) 1.0))) false false))
              (else
                (for (_array_element_7 _array_index_5) (Variables|/PremierLaserShow/Blueprints/BP_Spotlights.BP_Spotlights_C|GetSpotlightHingesHigher _returnvalue_2)
                  (Transformation|SetRelativeRotation _array_element_7 (Math|Rotator|MakeRotator (.roll (.rotation (Transformation|GetRelativeTransform _array_element_7))) (.pitch (.rotation (Transformation|GetRelativeTransform _array_element_7))) (.z (Math|Interpolation|VInterpTo (Math|Vector|MakeVector 0.0 0.0 (.yaw (.rotation (Transformation|GetRelativeTransform _array_element_7)))) (Math|Vector|MakeVector 0.0 0.0 (.yaw (Utilities|Array|Get(acopy) (Variables|Default|GetTransform%20Rotation) _array_index_5))) (Variables|Default|GetDelta%20Seconds) 1.0))) false false)))))
          (:then_5
            (if (Variables|Default|GetStartHeadControl)
              (for _array_element_8 (Variables|/PremierLaserShow/Blueprints/BP_Spotlights.BP_Spotlights_C|GetSpotlightBallsHigher _returnvalue_2)
                (bind _transform_10 (Default|GetHeadTransform (Variables|Default|GetBPI_Dancer)))
                (Transformation|SetRelativeRotation _array_element_8 (Math|Rotator|MakeRotator (.x (Math|Interpolation|VInterpTo (Math|Vector|MakeVector (.roll (.rotation (Transformation|GetRelativeTransform _array_element_8))) 0.0 0.0) (Math|Vector|MakeVector (- (.roll (.rotation _transform_10)) 9e+01) 0.0 0.0) (Variables|Default|GetDelta%20Seconds) 1.0)) (.pitch (.rotation (Transformation|GetRelativeTransform _array_element_8))) (.yaw (.rotation (Transformation|GetRelativeTransform _array_element_8)))) false false))
              (else
                (for (_array_element_9 _array_index_6) (Variables|/PremierLaserShow/Blueprints/BP_Spotlights.BP_Spotlights_C|GetSpotlightBallsHigher _returnvalue_2)
                  (Transformation|SetRelativeRotation _array_element_9 (Math|Rotator|MakeRotator (.x (Math|Interpolation|VInterpTo (Math|Vector|MakeVector (.roll (.rotation (Transformation|GetRelativeTransform _array_element_9))) 0.0 0.0) (Math|Vector|MakeVector (.pitch (Utilities|Array|Get(acopy) (Variables|Default|GetTransform%20Rotation) _array_index_6)) 0.0 0.0) (Variables|Default|GetDelta%20Seconds) 1.0)) (.pitch (.rotation (Transformation|GetRelativeTransform _array_element_9))) (.yaw (.rotation (Transformation|GetRelativeTransform _array_element_9)))) false false))))))))
    (:then_2
      (if (Variables|Default|GetEndSequence)
        (Utilities|FlowControl|DoOnce false :!label _label
          (:Completed
            (bind _newtrack_0 (Timeline|Timeline PlayFromStart)
              (:Update
                (Variables|Default|SetIntensityMin (Math|Float|Lerp 5e+01 0.0 _newtrack_0))
                (Variables|Default|SetIntensityMax (Math|Float|Lerp 2e+02 0.0 _newtrack_0)))
              (:Finished
                (Variables|Default|SetIntensityMin 0.0)
                (Variables|Default|SetIntensityMax 0.0)))))
        (else
          (goto _label Reset))))
    (:then_3
      (if (Variables|Default|GetRestart)
        (Variables|Default|SetStartBodyControl false)
        (Variables|Default|SetStartHeadControl false)
        (Variables|Default|SetEndSequence false)
        (Variables|Default|SetIntensityMin 5e+01)
        (Variables|Default|SetIntensityMax 2e+02)))))

(fn ConstructionScript)