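; Manager for a staged light show, driving the spotlights, circle projector, laser rig and maze projector in stages 1, 6, 8 and 9.
; Tick polls per-stage boolean cues and sets state on rigs found with GetActorOfClass, using DoOnce gates for one-shot triggers.
; Timelines run the Stage 1 closing rotation and color choreography and the Stage 6 and 8 transitions.
; BeginPlay caches the circle projector's starting intensity and cone brightness for its fades.
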(event EventBeginPlay
  (Utilities|FlowControl|Delay 0.2)
  (bind _returnvalue (Actor|GetActorOfClass "/PremierLaserShow/Blueprints/BP_CircleProjector_Part6.BP_CircleProjector_Part6_C"))
  (Variables|Default|SetStage6SpotlightStartIntensity (Variables|/PremierLaserShow/Blueprints/BP_CircleProjector_Part6.BP_CircleProjector_Part6_C|GetIntensity _returnvalue))
  (bind _returnvalue_2 (Rendering|Material|GetScalarParameterValue (Variables|/PremierLaserShow/Blueprints/BP_CircleProjector_Part6.BP_CircleProjector_Part6_C|GetConeMaterial _returnvalue) "BrightnessMultiplier" :!class /Script/Engine.MaterialInstanceDynamic))
  (Variables|Default|SetStage6BrightnessMultiplierStart _returnvalue_2))

(event EventTick
  (params (DeltaSeconds :type Float%20%28single-precision%29))
  (Utilities|FlowControl|Sequence
    (:then_1
      (Utilities|FlowControl|Sequence
        (:then_0
          (bind _returnvalue (Actor|GetActorOfClass "/PremierLaserShow/Blueprints/BP_Spotlights.BP_Spotlights_C"))
          (if (Variables|Stage1|GetStage1Start)
            (Utilities|FlowControl|DoOnce false :!label _label
              (:Completed
                (Variables|/PremierLaserShow/Blueprints/BP_Spotlights.BP_Spotlights_C|SetRandomLight _returnvalue true)))
            (else
              (goto _label Reset))))
        (:then_1
          (bind _returnvalue_2 (Actor|GetActorOfClass "/PremierLaserShow/Blueprints/BP_Spotlights.BP_Spotlights_C"))
          (if (Variables|Stage1|GetStage1MultiLights)
            (Utilities|FlowControl|DoOnce false :!label _label_2
              (:Completed
                (Variables|Stage1|SetStage1Start false)
                (Variables|/PremierLaserShow/Blueprints/BP_Spotlights.BP_Spotlights_C|SetRandomLight _returnvalue_2 false)
                (Variables|/PremierLaserShow/Blueprints/BP_Spotlights.BP_Spotlights_C|SetMultipleLightsAllowed _returnvalue_2 true)
                (Variables|/PremierLaserShow/Blueprints/BP_Spotlights.BP_Spotlights_C|SetTurnOnAllLights _returnvalue_2 true)))
            (else
              (goto _label_2 Reset))))
        (:then_2
          (bind _returnvalue_3 (Actor|GetActorOfClass "/PremierLaserShow/Blueprints/BP_Spotlights.BP_Spotlights_C"))
          (if (Variables|Stage1|GetStage1SwitchToLHand)
            (Utilities|FlowControl|DoOnce false :!label _label_3
              (:Completed
                (Variables|/PremierLaserShow/Blueprints/BP_Spotlights.BP_Spotlights_C|SetLHandActive _returnvalue_3 true)
                (Variables|Stage1|SetStage1SwitchToLHand false)))
            (else
              (goto _label_3 Reset))))
        (:then_3
          (bind _returnvalue_4 (Actor|GetActorOfClass "/PremierLaserShow/Blueprints/BP_Spotlights.BP_Spotlights_C"))
          (if (Variables|Stage1|GetStage1SwitchToRHand)
            (Utilities|FlowControl|DoOnce false :!label _label_4
              (:Completed
                (Variables|/PremierLaserShow/Blueprints/BP_Spotlights.BP_Spotlights_C|SetRHandActive _returnvalue_4 true)
                (Variables|Stage1|SetStage1SwitchToRHand false)))
            (else
              (goto _label_4 Reset))))
        (:then_4
          (bind _returnvalue_5 (Actor|GetActorOfClass "/PremierLaserShow/Blueprints/BP_Spotlights.BP_Spotlights_C"))
          (if (Variables|Stage1|GetStage1SwitchToRFoot)
            (Utilities|FlowControl|DoOnce false :!label _label_5
              (:Completed
                (Variables|/PremierLaserShow/Blueprints/BP_Spotlights.BP_Spotlights_C|SetRToeActive _returnvalue_5 true)
                (Variables|Stage1|SetStage1SwitchToRFoot false)))
            (else
              (goto _label_5 Reset))))
        (:then_5
          (bind _returnvalue_6 (Actor|GetActorOfClass "/PremierLaserShow/Blueprints/BP_Spotlights.BP_Spotlights_C"))
          (if (Variables|Stage1|GetStage1RandomBones)
            (Utilities|FlowControl|DoOnce false :!label _label_6
              (:Completed
                (Variables|/PremierLaserShow/Blueprints/BP_Spotlights.BP_Spotlights_C|SetRandomiseTarget _returnvalue_6 true)))
            (else
              (goto _label_6 Reset))))
        (:then_6
          (bind _returnvalue_7 (Actor|GetActorOfClass "/PremierLaserShow/Blueprints/BP_Spotlights.BP_Spotlights_C"))
          (if (Variables|Stage1|GetStage1MultiRandomBones)
            (Utilities|FlowControl|DoOnce false :!label _label_7
              (:Completed
                (Variables|Stage1|SetStage1RandomBones false)
                (Variables|/PremierLaserShow/Blueprints/BP_Spotlights.BP_Spotlights_C|SetRandomiseTarget _returnvalue_7 false)
                (Utilities|FlowControl|Delay 3.0)
                (Variables|/PremierLaserShow/Blueprints/BP_Spotlights.BP_Spotlights_C|SetOneTarget _returnvalue_7 false)
                (Utilities|FlowControl|Delay 3.0)
                (Variables|/PremierLaserShow/Blueprints/BP_Spotlights.BP_Spotlights_C|SetRandomiseTarget _returnvalue_7 true)))
            (else
              (goto _label_7 Reset))))
        (:then_7
          (bind _returnvalue_8 (Actor|GetActorOfClass "/PremierLaserShow/Blueprints/BP_Spotlights.BP_Spotlights_C"))
          (if (Variables|Stage1|GetStage1End)
            (Utilities|FlowControl|DoOnce false :!label _label_8
              (:Completed
                (for _array_element (Variables|/PremierLaserShow/Blueprints/BP_Spotlights.BP_Spotlights_C|GetRandomBoneIntegerArray _returnvalue_8)
                  (Utilities|Array|SetArrayElem (Variables|/PremierLaserShow/Blueprints/BP_Spotlights.BP_Spotlights_C|GetRandomBoneIntegerArray _returnvalue_8) _array_element _array_element))
                (Variables|/PremierLaserShow/Blueprints/BP_Spotlights.BP_Spotlights_C|SetRandomiseTarget _returnvalue_8 false)
                (Variables|Stage1|SetStage1MultiRandomBones false)
                (Utilities|FlowControl|Delay 3.0)
                (Variables|/PremierLaserShow/Blueprints/BP_Spotlights.BP_Spotlights_C|SetEndSequence _returnvalue_8 true)
                (Utilities|FlowControl|Sequence
                  (:then_0
                    (bind _newtrack_0 (Timeline|Stage1EndSequence PlayFromStart)
                      (:Update
                        (Utilities|FlowControl|Sequence
                          (:then_0
                            (for _array_element_2 (Variables|/PremierLaserShow/Blueprints/BP_Spotlights.BP_Spotlights_C|GetSpotlightHinges _returnvalue_8)
                              (Transformation|SetRelativeRotation _array_element_2 (Math|Rotator|Lerp(Rotator) (Variables|/Script/Engine.SceneComponent|GetRelativeRotation _array_element_2) "0, 0, 0" _newtrack_0) false false)))
                          (:then_1
                            (for _array_element_3 (Variables|/PremierLaserShow/Blueprints/BP_Spotlights.BP_Spotlights_C|GetSpotlightBalls _returnvalue_8)
                              (Transformation|SetRelativeRotation _array_element_3 (Math|Rotator|Lerp(Rotator) (Variables|/Script/Engine.SceneComponent|GetRelativeRotation _array_element_3) "0.000000,0.000000,-45.000000" _newtrack_0) false false)))))
                      (:Finished
                        (Utilities|FlowControl|Sequence
                          (:then_0
                            (for _array_element_4 (Variables|/PremierLaserShow/Blueprints/BP_Spotlights.BP_Spotlights_C|GetSpotlightHinges _returnvalue_8)
                              (Transformation|SetRelativeRotation _array_element_4 "0, 0, 0" false false)))
                          (:then_1
                            (for _array_element_5 (Variables|/PremierLaserShow/Blueprints/BP_Spotlights.BP_Spotlights_C|GetSpotlightBalls _returnvalue_8)
                              (Transformation|SetRelativeRotation _array_element_5 "0.000000,0.000000,-45.000000" false false)))
                          (:then_2
                            (Utilities|FlowControl|Delay 5.0)
                            (bind _newtrack_0_2 (Timeline|Timeline_0 PlayFromStart)
                              (:Update
                                (Utilities|FlowControl|Sequence
                                  (:then_0
                                    (for _array_element_6 (Variables|/PremierLaserShow/Blueprints/BP_Spotlights.BP_Spotlights_C|GetSpotlightHinges _returnvalue_8)
                                      (Transformation|SetRelativeRotation _array_element_6 (Math|Rotator|Lerp(Rotator) "0, 0, 0" "0.000000,-90.000000,0.000000" _newtrack_0_2) false false)))
                                  (:then_1
                                    (for _array_element_7 (Variables|/PremierLaserShow/Blueprints/BP_Spotlights.BP_Spotlights_C|GetSpotlightBalls _returnvalue_8)
                                      (Transformation|SetRelativeRotation _array_element_7 (Math|Rotator|Lerp(Rotator) "0.000000,0.000000,-45.000000" "0.000000,0.000000,-60.000000" _newtrack_0_2) false false)))))
                              (:Finished
                                (bind _newtrack_0_3 (Timeline|Timeline_2 PlayFromStart)
                                  (:Update
                                    (Rendering|Components|Light|SetLightColor (Variables|/PremierLaserShow/Blueprints/BP_Spotlights.BP_Spotlights_C|GetSpotLight_09 _returnvalue_8) (Math|Color|Lerp(LinearColor) "(R=1.000000,G=1.000000,B=1.000000,A=1.000000)" "(R=0.049707,G=0.401978,B=1.000000,A=1.000000)" _newtrack_0_3) true))
                                  (:Finished
                                    (Utilities|FlowControl|Delay 2.0)
                                    (bind (_direction _newtrack_0_4 _newtrack_1) (Timeline|Timeline_3 PlayFromStart)
                                      (:Update
                                        (Utilities|FlowControl|Sequence
                                          (:then_0
                                            (for _array_element_8 (Variables|/PremierLaserShow/Blueprints/BP_Spotlights.BP_Spotlights_C|GetSpotlightHinges _returnvalue_8)
                                              (Transformation|SetRelativeRotation _array_element_8 (Math|Rotator|Lerp(Rotator) "0, 0, 0" "0.000000,-90.000000,0.000000" _newtrack_0_4) false false)))
                                          (:then_1
                                            (for _array_element_9 (Variables|/PremierLaserShow/Blueprints/BP_Spotlights.BP_Spotlights_C|GetSpotlightBalls _returnvalue_8)
                                              (Transformation|SetRelativeRotation _array_element_9 (Math|Rotator|Lerp(Rotator) "0.000000,0.000000,-45.000000" "0.000000,0.000000,-60.000000" _newtrack_1) false false)))))
                                      (:Finished
                                        (bind _newtrack_0_5 (Timeline|Timeline_1 PlayFromStart)
                                          (:Update
                                            (Utilities|FlowControl|Sequence
                                              (:then_0
                                                (for _array_element_10 (Variables|/PremierLaserShow/Blueprints/BP_Spotlights.BP_Spotlights_C|GetSpotlightHinges _returnvalue_8)
                                                  (Transformation|SetRelativeRotation _array_element_10 (Math|Rotator|Lerp(Rotator) "0, 0, 0" "0, 0, 0" _newtrack_0_5) false false)))
                                              (:then_1
                                                (for _array_element_11 (Variables|/PremierLaserShow/Blueprints/BP_Spotlights.BP_Spotlights_C|GetSpotlightBalls _returnvalue_8)
                                                  (Transformation|SetRelativeRotation _array_element_11 (Math|Rotator|Lerp(Rotator) "0.000000,0.000000,-45.000000" "0.000000,0.000000,10.000000" _newtrack_0_5) false false)))))
                                          (:Finished
                                            (Utilities|FlowControl|Sequence
                                              (:then_0
                                                (for _array_element_12 (Variables|/PremierLaserShow/Blueprints/BP_Spotlights.BP_Spotlights_C|GetSpotlightHinges _returnvalue_8)
                                                  (Transformation|SetRelativeRotation _array_element_12 "0, 0, 0" false false)))
                                              (:then_1
                                                (for _array_element_13 (Variables|/PremierLaserShow/Blueprints/BP_Spotlights.BP_Spotlights_C|GetSpotlightBalls _returnvalue_8)
                                                  (Transformation|SetRelativeRotation _array_element_13 "0.000000,0.000000,10.000000" false false)))
                                              (:then_2)))))))))))))))
                  (:then_1
                    (for (_ _array_index) (Variables|/PremierLaserShow/Blueprints/BP_Spotlights.BP_Spotlights_C|GetCurrentRandomPositionArray _returnvalue_8)
                      (Utilities|Array|SetArrayElem (Variables|/PremierLaserShow/Blueprints/BP_Spotlights.BP_Spotlights_C|GetCurrentRandomPositionArray _returnvalue_8) _array_index "0.000000,0.000000,200.000000"))))))
            (else
              (goto _label_8 Reset))))))
    (:then_6
      ;[1 1 1 1 50] Part 6: Circle Projector
      (Utilities|FlowControl|Sequence
        (:then_0
          (if (Variables|Stage6|GetStage6-Start)
            (Utilities|FlowControl|DoOnce false :!label _label_9
              (:Completed
                (bind _newtrack_0_6 (Timeline|Stage%206%20Triggered PlayFromStart)
                  (:Update
                    (bind _returnvalue_9 (Actor|GetActorOfClass "/PremierLaserShow/Blueprints/BP_CircleProjector_Part6.BP_CircleProjector_Part6_C"))
                    (Variables|/PremierLaserShow/Blueprints/BP_CircleProjector_Part6.BP_CircleProjector_Part6_C|SetRadialCoverAmount _returnvalue_9 _newtrack_0_6)
                    (if (> _newtrack_0_6 0.01)
                      (Variables|/PremierLaserShow/Blueprints/BP_CircleProjector_Part6.BP_CircleProjector_Part6_C|SetIntensity _returnvalue_9 (Variables|Default|GetStage6SpotlightStartIntensity))
                      (Rendering|Material|SetScalarParameterValue (Variables|/PremierLaserShow/Blueprints/BP_CircleProjector_Part6.BP_CircleProjector_Part6_C|GetConeMaterial _returnvalue_9) "BrightnessMultiplier" (Variables|Default|GetStage6BrightnessMultiplierStart) :!class /Script/Engine.MaterialInstanceDynamic)))
                  (:Finished
                    (Variables|Stage6|SetStage6-Start false)
                    (goto _label_9 Reset)))))))
        (:then_1
          (bind _returnvalue_10 (Actor|GetActorOfClass "/PremierLaserShow/Blueprints/BP_CircleProjector_Part6.BP_CircleProjector_Part6_C"))
          (Variables|/PremierLaserShow/Blueprints/BP_CircleProjector_Part6.BP_CircleProjector_Part6_C|SetIsDancerInfluencing _returnvalue_10 (Variables|Stage6|GetStage6-ArmsInfluenceCircle)))
        (:then_2
          (bind _returnvalue_11 (Actor|GetActorOfClass "/PremierLaserShow/Blueprints/BP_CircleProjector_Part6.BP_CircleProjector_Part6_C"))
          (Variables|/PremierLaserShow/Blueprints/BP_CircleProjector_Part6.BP_CircleProjector_Part6_C|SetIsSplitLaserTime _returnvalue_11 (Variables|Stage6|GetStage6-SplitLaserTime)))
        (:then_3
          (if (Variables|Stage6|GetStage6-End)
            (Utilities|FlowControl|DoOnce false :!label _label_10
              (:Completed
                (bind _newtrack_0_7 (Timeline|Stage%206%20Fadeout PlayFromStart)
                  (:Update
                    (bind _returnvalue_12 (Actor|GetActorOfClass "/PremierLaserShow/Blueprints/BP_CircleProjector_Part6.BP_CircleProjector_Part6_C"))
                    (Variables|/PremierLaserShow/Blueprints/BP_CircleProjector_Part6.BP_CircleProjector_Part6_C|SetIntensity _returnvalue_12 (* (Variables|Default|GetStage6SpotlightStartIntensity) _newtrack_0_7))
                    (Rendering|Material|SetScalarParameterValue (Variables|/PremierLaserShow/Blueprints/BP_CircleProjector_Part6.BP_CircleProjector_Part6_C|GetConeMaterial _returnvalue_12) "BrightnessMultiplier" (* (Variables|Default|GetStage6BrightnessMultiplierStart) _newtrack_0_7) :!class /Script/Engine.MaterialInstanceDynamic))
                  (:Finished
                    (Variables|Stage6|SetStage6-End false)
                    (goto _label_10 Reset)))))))))
    (:then_8
      (Utilities|FlowControl|Sequence
        (:then_0
          (if (Variables|Stage8|GetStage8-Start)
            (bind _returnvalue_13 (Actor|GetActorOfClass "/PremierLaserShow/Blueprints/BP_LaserRig_Part8.BP_LaserRig_Part8_C"))
            (Variables|/PremierLaserShow/Blueprints/BP_LaserRig_Part8.BP_LaserRig_Part8_C|SetIsTracking _returnvalue_13 true)
            (Utilities|FlowControl|DoOnce false :!label _label_11
              (:Completed
                (bind _newtrack_0_8 (Timeline|Stage%208%20Triggered PlayFromStart)
                  (:Update
                    (bind _returnvalue_14 (Actor|GetActorOfClass "/PremierLaserShow/Blueprints/BP_LaserRig_Part8.BP_LaserRig_Part8_C"))
                    (Variables|/PremierLaserShow/Blueprints/BP_LaserRig_Part8.BP_LaserRig_Part8_C|SetLaserMaterialIntensity _returnvalue_14 _newtrack_0_8))
                  (:Finished
                    (Variables|Stage8|SetStage8-Start false)
                    (goto _label_11 Reset)))))))
        (:then_1
          (if (Variables|Stage8|GetStage8-LaserDance)
            (bind _returnvalue_15 (Actor|GetActorOfClass "/PremierLaserShow/Blueprints/BP_LaserRig_Part8.BP_LaserRig_Part8_C"))
            (Utilities|IsValid _returnvalue_15
              (:Is%20Valid
                (Variables|/PremierLaserShow/Blueprints/BP_LaserRig_Part8.BP_LaserRig_Part8_C|SetFinalSequence _returnvalue_15 true)))
            (else
              (bind _returnvalue_16 (Actor|GetActorOfClass "/PremierLaserShow/Blueprints/BP_LaserRig_Part8.BP_LaserRig_Part8_C"))
              (Utilities|IsValid _returnvalue_16
                (:Is%20Valid
                  (Variables|/PremierLaserShow/Blueprints/BP_LaserRig_Part8.BP_LaserRig_Part8_C|SetFinalSequence _returnvalue_16 false))))))
        (:then_2
          (bind _returnvalue_17 (Actor|GetActorOfClass "/PremierLaserShow/Blueprints/BP_LaserRig_Part8.BP_LaserRig_Part8_C"))
          (if (Variables|/PremierLaserShow/Blueprints/BP_LaserRig_Part8.BP_LaserRig_Part8_C|GetFinalSequenceFadeoutPossible _returnvalue_17)
            (if (Variables|Stage8|GetStage8-FadeOut)
              (Utilities|FlowControl|DoOnce false :!label _label_12
                (:Completed
                  (bind _newtrack_0_9 (Timeline|Timeline PlayFromStart)
                    (:Update
                      (Variables|/PremierLaserShow/Blueprints/BP_LaserRig_Part8.BP_LaserRig_Part8_C|SetLaserMaterialIntensity _returnvalue_17 _newtrack_0_9))
                    (:Finished
                      (Variables|Stage8|SetStage8-FadeOut false)
                      (Variables|/PremierLaserShow/Blueprints/BP_LaserRig_Part8.BP_LaserRig_Part8_C|SetIsTracking _returnvalue_17 false)
                      (goto _label_12 Reset))))))))))
    (:then_9
      (Utilities|FlowControl|Sequence
        (:then_0
          (if (Variables|Stage9|GetStage9-Start)
            (bind _returnvalue_18 (Actor|GetActorOfClass "/PremierLaserShow/Blueprints/BP_MazeProjector_Part9.BP_MazeProjector_Part9_C"))
            (Variables|/PremierLaserShow/Blueprints/BP_MazeProjector_Part9.BP_MazeProjector_Part9_C|SetStartLights _returnvalue_18 true)))
        (:then_1
          (if (Variables|Stage9|GetStage9-Maze1)
            (bind _returnvalue_19 (Actor|GetActorOfClass "/PremierLaserShow/Blueprints/BP_MazeProjector_Part9.BP_MazeProjector_Part9_C"))
            (Variables|/PremierLaserShow/Blueprints/BP_MazeProjector_Part9.BP_MazeProjector_Part9_C|SetStartStage1 _returnvalue_19 true)))
        (:then_2
          (if (Variables|Stage9|GetStage9-Maze2)
            (bind _returnvalue_20 (Actor|GetActorOfClass "/PremierLaserShow/Blueprints/BP_MazeProjector_Part9.BP_MazeProjector_Part9_C"))
            (Variables|/PremierLaserShow/Blueprints/BP_MazeProjector_Part9.BP_MazeProjector_Part9_C|SetStartStage2 _returnvalue_20 true)))
        (:then_3
          (if (Variables|Stage9|GetStage9-Maze3)
            (bind _returnvalue_21 (Actor|GetActorOfClass "/PremierLaserShow/Blueprints/BP_MazeProjector_Part9.BP_MazeProjector_Part9_C"))
            (Variables|/PremierLaserShow/Blueprints/BP_MazeProjector_Part9.BP_MazeProjector_Part9_C|SetStartStage3 _returnvalue_21 true)))
        (:then_4
          (if (Variables|Stage9|GetStage9-FinalSequence)
            (bind _returnvalue_22 (Actor|GetActorOfClass "/PremierLaserShow/Blueprints/BP_MazeProjector_Part9.BP_MazeProjector_Part9_C"))
            (Variables|/PremierLaserShow/Blueprints/BP_MazeProjector_Part9.BP_MazeProjector_Part9_C|SetFinalStage _returnvalue_22 true)))))))

(fn ConstructionScript)