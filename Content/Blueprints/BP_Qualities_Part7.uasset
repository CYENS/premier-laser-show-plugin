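; BP_Qualities_Part7 drives the BP_Spotlights rig with randomised swivelling and blue lighting that reacts to a dancer's movement.
; Each tick it turns eight arm, hand, leg and toe velocities into intensities, applied to both tiers while StartGenerating is on.
; Per-light random timers pick new angles, blended toward stabilised values by per-tier alphas.
; Hinge yaw and ball roll interpolate between previous and new angles over each interval.
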(event Custom|ChangeTimer
  (params (Index :type Integer))
  (bind _stabalisealphalower (Variables|Default|GetStabaliseAlphaLower))
  (bind _stabalisealphaupper (Variables|Default|GetStabaliseAlphaUpper))
  (Utilities|Array|SetArrayElem (Variables|Default|GetRandomFloats) Index (+ (Variables|Default|GetDelta%20Seconds) (Math|Random|RandomFloatinRange (Variables|Default|GetTimeMin) (Variables|Default|GetTimeMax))))
  (Utilities|Array|SetArrayElem (Variables|Default|GetPreviousRotations) Index (Utilities|Array|Get(acopy) (Variables|Default|GetRandomRotations) Index) true)
  (Utilities|Array|SetArrayElem (Variables|Default|GetTimesStart) Index (- (Utilities|Array|Get(acopy) (Variables|Default|GetRandomFloats) Index) (Variables|Default|GetDelta%20Seconds)) true)
  (if (<= Index 7)
    (Utilities|Array|SetArrayElem (Variables|Default|GetRandomRotations) Index (Math|Rotator|MakeRotator (Math|Float|Lerp (Math|Random|RandomFloatinRange (Variables|Default|GetRotationMin) (Variables|Default|GetRotationMax)) (Variables|Default|GetStabalisedXLower) _stabalisealphalower) 0.0 (Math|Float|Lerp (Math|Random|RandomFloatinRange (Variables|Default|GetRotationMin) (Variables|Default|GetRotationMax)) (Variables|Default|GetStabalisedZLower) _stabalisealphalower)) true)
    (else
      (Utilities|Array|SetArrayElem (Variables|Default|GetRandomRotations) Index (Math|Rotator|MakeRotator (Math|Float|Lerp (Math|Random|RandomFloatinRange (Variables|Default|GetRotationMin) (Variables|Default|GetRotationMax)) (Variables|Default|GetStabalisedXUpper) _stabalisealphaupper) 0.0 (Math|Float|Lerp (Math|Random|RandomFloatinRange (Variables|Default|GetRotationMin) (Variables|Default|GetRotationMax)) (Variables|Default|GetStabalisedZUpper) _stabalisealphaupper)) true))))

(event EventBeginPlay
  (Utilities|FlowControl|Sequence
    (:then_0
      (bind _returnvalue (Actor|GetActorOfClass "/PremierLaserShow/Blueprints/BP_Spotlights.BP_Spotlights_C"))
      (Variables|Default|SetSpotlight%20Hinges%20Lower (Variables|/PremierLaserShow/Blueprints/BP_Spotlights.BP_Spotlights_C|GetSpotlightHingesLower _returnvalue))
      (Variables|Default|SetSpotlight%20Hinges%20Higher (Variables|/PremierLaserShow/Blueprints/BP_Spotlights.BP_Spotlights_C|GetSpotlightHingesHigher _returnvalue))
      (Variables|Default|SetSpotlight%20Balls%20Lower (Variables|/PremierLaserShow/Blueprints/BP_Spotlights.BP_Spotlights_C|GetSpotlightBallsLower _returnvalue))
      (Variables|Default|SetSpotlight%20Balls%20Higher (Variables|/PremierLaserShow/Blueprints/BP_Spotlights.BP_Spotlights_C|GetSpotlightBallsHigher _returnvalue)))))

(event EventTick
  (params (DeltaSeconds :type Float%20%28single-precision%29))
  (bind _randomfloats (Variables|Default|GetRandomFloats))
  (Variables|Default|SetDelta%20Seconds (+ DeltaSeconds (Variables|Default|GetDelta%20Seconds)))
  (Utilities|FlowControl|Sequence
    (:then_0
      (if (Variables|Default|GetDancerFound)
        (Utilities|FlowControl|Sequence
          (:then_0
            (bind _velocity (Default|GetLForeArmVelocity (Variables|Default|GetBPI_Dancer)))
            (Utilities|Array|SetArrayElem (Variables|Default|GetVelocities) 0 (Math|Vector|MakeVector (Math|Float|Absolute(Float) (.x _velocity)) (Math|Float|Absolute(Float) (.y _velocity)) (Math|Float|Absolute(Float) (.z _velocity))) true)
            (bind _velocity_2 (Default|GetLHandVelocity (Variables|Default|GetBPI_Dancer)))
            (Utilities|Array|SetArrayElem (Variables|Default|GetVelocities) 1 (Math|Vector|MakeVector (Math|Float|Absolute(Float) (.x _velocity_2)) (Math|Float|Absolute(Float) (.y _velocity_2)) (Math|Float|Absolute(Float) (.z _velocity_2))) true)
            (bind _velocity_3 (Default|GetLLegVelocity (Variables|Default|GetBPI_Dancer)))
            (Utilities|Array|SetArrayElem (Variables|Default|GetVelocities) 2 (Math|Vector|MakeVector (Math|Float|Absolute(Float) (.x _velocity_3)) (Math|Float|Absolute(Float) (.y _velocity_3)) (Math|Float|Absolute(Float) (.z _velocity_3))) true)
            (bind _velocity_4 (Default|GetLToeVelocity (Variables|Default|GetBPI_Dancer)))
            (Utilities|Array|SetArrayElem (Variables|Default|GetVelocities) 3 (Math|Vector|MakeVector (Math|Float|Absolute(Float) (.x _velocity_4)) (Math|Float|Absolute(Float) (.y _velocity_4)) (Math|Float|Absolute(Float) (.z _velocity_4))) true)
            (bind _velocity_5 (Default|GetRForeArmVelocity (Variables|Default|GetBPI_Dancer)))
            (Utilities|Array|SetArrayElem (Variables|Default|GetVelocities) 4 (Math|Vector|MakeVector (Math|Float|Absolute(Float) (.x _velocity_5)) (Math|Float|Absolute(Float) (.y _velocity_5)) (Math|Float|Absolute(Float) (.z _velocity_5))) true)
            (bind _velocity_6 (Default|GetRHandVelocity (Variables|Default|GetBPI_Dancer)))
            (Utilities|Array|SetArrayElem (Variables|Default|GetVelocities) 5 (Math|Vector|MakeVector (Math|Float|Absolute(Float) (.x _velocity_6)) (Math|Float|Absolute(Float) (.y _velocity_6)) (Math|Float|Absolute(Float) (.z _velocity_6))) true)
            (bind _velocity_7 (Default|GetRLegVelocity (Variables|Default|GetBPI_Dancer)))
            (Utilities|Array|SetArrayElem (Variables|Default|GetVelocities) 6 (Math|Vector|MakeVector (Math|Float|Absolute(Float) (.x _velocity_7)) (Math|Float|Absolute(Float) (.y _velocity_7)) (Math|Float|Absolute(Float) (.z _velocity_7))) true)
            (bind _velocity_8 (Default|GetRToeVelocity (Variables|Default|GetBPI_Dancer)))
            (Utilities|Array|SetArrayElem (Variables|Default|GetVelocities) 7 (Math|Vector|MakeVector (Math|Float|Absolute(Float) (.x _velocity_8)) (Math|Float|Absolute(Float) (.y _velocity_8)) (Math|Float|Absolute(Float) (.z _velocity_8))) true))
          (:then_1
            (for (_array_element _array_index) (Variables|Default|GetVelocities)
              (Utilities|Array|SetArrayElem (Variables|Default|GetIntensities) _array_index (* (Math|Float|Sqrt (Math|Vector|GetMaxElement _array_element)) 2e+02) true))))
        (else
          (bind _returnvalue (Actor|GetActorOfClass "/PremierLaserShow/Blueprints/BP_Spotlights.BP_Spotlights_C"))
          (bind _output_get (Variables|Default|SetBPI_Dancer (Variables|/PremierLaserShow/Blueprints/BP_Spotlights.BP_Spotlights_C|GetDancerSkeleton _returnvalue)))
          (Utilities|IsValid (Utilities|ToObject(Interface) _output_get)
            (:Is%20Valid
              (Variables|Default|SetDancerFound true))))))
    (:then_2
      (Utilities|FlowControl|Sequence
        (:then_0
          (for (_array_element_2 _array_index_2) (Variables|Default|GetSpotlight%20Hinges%20Lower)
            (Transformation|SetRelativeRotation _array_element_2 (Math|Rotator|MakeRotator 0.0 0.0 (.yaw (Math|Rotator|Lerp(Rotator) (Utilities|Array|Get(acopy) (Variables|Default|GetPreviousRotations) _array_index_2) (Utilities|Array|Get(acopy) (Variables|Default|GetRandomRotations) _array_index_2) (- 1.0 (/ (Utilities|Array|Get(acopy) (Variables|Default|GetTimes) _array_index_2) (Utilities|Array|Get(acopy) (Variables|Default|GetTimesStart) _array_index_2))) true))) false false)))
        (:then_1
          (for (_array_element_3 _array_index_3) (Variables|Default|GetSpotlight%20Hinges%20Higher)
            (Transformation|SetRelativeRotation _array_element_3 (Math|Rotator|MakeRotator 0.0 0.0 (.yaw (Math|Rotator|Lerp(Rotator) (Utilities|Array|Get(acopy) (Variables|Default|GetPreviousRotations) (+ _array_index_3 8)) (Utilities|Array|Get(acopy) (Variables|Default|GetRandomRotations) (+ _array_index_3 8)) (- 1.0 (/ (Utilities|Array|Get(acopy) (Variables|Default|GetTimes) (+ _array_index_3 8)) (Utilities|Array|Get(acopy) (Variables|Default|GetTimesStart) (+ _array_index_3 8)))) true))) false false)))
        (:then_2
          (for (_array_element_4 _array_index_4) (Variables|Default|GetSpotlight%20Balls%20Lower)
            (Transformation|SetRelativeRotation _array_element_4 (Math|Rotator|MakeRotator (.roll (Math|Rotator|Lerp(Rotator) (Utilities|Array|Get(acopy) (Variables|Default|GetPreviousRotations) _array_index_4) (Utilities|Array|Get(acopy) (Variables|Default|GetRandomRotations) _array_index_4) (- 1.0 (/ (Utilities|Array|Get(acopy) (Variables|Default|GetTimes) _array_index_4) (Utilities|Array|Get(acopy) (Variables|Default|GetTimesStart) _array_index_4))) true)) 0.0 0.0) false false)))
        (:then_3
          (for (_array_element_5 _array_index_5) (Variables|Default|GetSpotlight%20Balls%20Higher)
            (Transformation|SetRelativeRotation _array_element_5 (Math|Rotator|MakeRotator (.roll (Math|Rotator|Lerp(Rotator) (Utilities|Array|Get(acopy) (Variables|Default|GetPreviousRotations) (+ _array_index_5 8)) (Utilities|Array|Get(acopy) (Variables|Default|GetRandomRotations) (+ _array_index_5 8)) (- 1.0 (/ (Utilities|Array|Get(acopy) (Variables|Default|GetTimes) (+ _array_index_5 8)) (Utilities|Array|Get(acopy) (Variables|Default|GetTimesStart) (+ _array_index_5 8)))) true)) 0.0 0.0) false false)))))
    (:then_3
      (if (Variables|Default|GetStartGenerating)
        (Utilities|FlowControl|Sequence
          (:then_0
            (Utilities|FlowControl|DoOnce false :!label _label
              (:Completed
                (Utilities|FlowControl|Sequence
                  (:then_0
                    (Variables|Default|SetFirstTimesSet false)
                    (for (_ _array_index_6) _randomfloats
                      (Utilities|Array|SetArrayElem _randomfloats _array_index_6 (+ (Variables|Default|GetDelta%20Seconds) (Math|Random|RandomFloatinRange (Variables|Default|GetTimeMin) (Variables|Default|GetTimeMax)))))
                    (Variables|Default|SetFirstTimesSet true))
                  (:then_1
                    (bind _returnvalue_2 (Actor|GetActorOfClass "/PremierLaserShow/Blueprints/BP_Spotlights.BP_Spotlights_C"))
                    (Utilities|FlowControl|Sequence
                      (:then_0
                        (Variables|/PremierLaserShow/Blueprints/BP_Spotlights.BP_Spotlights_C|SetCircumventOrder _returnvalue_2 true))
                      (:then_1
                        (for _array_element_6 (Variables|/PremierLaserShow/Blueprints/BP_Spotlights.BP_Spotlights_C|GetSpotlightsHigher _returnvalue_2)
                          (Rendering|Components|Light|SetIntensity _array_element_6 1e+02)
                          (Rendering|Components|Light|SetLightColor _array_element_6 "(R=0.049707,G=0.401978,B=1.000000,A=1.000000)" true)))
                      (:then_2
                        (for _array_element_7 (Variables|/PremierLaserShow/Blueprints/BP_Spotlights.BP_Spotlights_C|GetSpotlightsLower _returnvalue_2)
                          (Rendering|Components|Light|SetIntensity _array_element_7 1e+02)
                          (Rendering|Components|Light|SetLightColor _array_element_7 "(R=0.049707,G=0.401978,B=1.000000,A=1.000000)" true)))))))))
          (:then_1
            (if (Variables|Default|GetFirstTimesSet)
              (Utilities|FlowControl|Sequence
                (:then_0
                  (for (_array_element_8 _array_index_7) (Variables|Default|GetRandomFloats)
                    (Utilities|Array|SetArrayElem (Variables|Default|GetTimes) _array_index_7 (- _array_element_8 (Variables|Default|GetDelta%20Seconds)))))
                (:then_1
                  (for (_array_element_9 _array_index_8) (Variables|Default|GetRandomFloats)
                    (if (<= _array_element_9 (Variables|Default|GetDelta%20Seconds))
                      (CallFunction|ChangeTimer _array_index_8))))
                (:then_2
                  (bind _returnvalue_3 (Actor|GetActorOfClass "/PremierLaserShow/Blueprints/BP_Spotlights.BP_Spotlights_C"))
                  (Utilities|FlowControl|Sequence
                    (:then_0
                      (for (_array_element_10 _array_index_9) (Variables|/PremierLaserShow/Blueprints/BP_Spotlights.BP_Spotlights_C|GetSpotlightsHigher _returnvalue_3)
                        (Rendering|Components|Light|SetIntensity _array_element_10 (Utilities|Array|Get(acopy) (Variables|Default|GetIntensities) _array_index_9))
                        (Rendering|Components|Light|SetLightColor _array_element_10 "(R=0.049707,G=0.401978,B=1.000000,A=1.000000)" true)))
                    (:then_1
                      (for (_array_element_11 _array_index_10) (Variables|/PremierLaserShow/Blueprints/BP_Spotlights.BP_Spotlights_C|GetSpotlightsLower _returnvalue_3)
                        (Rendering|Components|Light|SetIntensity _array_element_11 (Utilities|Array|Get(acopy) (Variables|Default|GetIntensities) _array_index_10))
                        (Rendering|Components|Light|SetLightColor _array_element_11 "(R=0.049707,G=0.401978,B=1.000000,A=1.000000)" true)))))))))
        (else
          (goto _label Reset))))))

(fn ConstructionScript)