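; BP_SpotlightHinge is the swivel part of a spotlight that turns to follow a target actor.
; On BeginPlay it picks one random BP_SpotlightLookAt actor from the level and keeps it as its target.
; Each Tick it interpolates toward the look-at rotation with RInterpTo at a Speed variable, applying only the yaw so the hinge rotates around the vertical axis.
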(event EventBeginPlay
  (bind _outactors (Actor|GetAllActorsOfClass "/PremierLaserShow/Blueprints/BP_SpotlightLookAt.BP_SpotlightLookAt_C"))
  (Variables|Default|SetLookAtActor (.OutItem (Utilities|Array|Random _outactors))))

(event Collision|EventActorBeginOverlap
  (params (OtherActor :type Actor%20Object%20Reference)))

(event EventTick
  (params (DeltaSeconds :type Float%20%28single-precision%29))
  (Transformation|SetActorRotation (Math|Rotator|MakeRotator 0.0 0.0 (.yaw (Math|Interpolation|RInterpTo (Transformation|GetActorRotation) (Math|Rotator|FindLookatRotation (Transformation|GetActorLocation) (Transformation|GetActorLocation (Variables|Default|GetLookAtActor))) (Utilities|Time|GetWorldDeltaSeconds) (Variables|Default|GetSpeed))))))

(fn ConstructionScript)