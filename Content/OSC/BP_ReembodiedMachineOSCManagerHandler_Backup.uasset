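; OSC handler that turns scene and phase activations into cue flags on BP_PremierSequenceManager for a staged light and laser show.
; Scene activations from ReembodiedMachineOscHandler fire a dispatcher, then a per-scene switch sets the matching Stage booleans, printing unknown combinations.
; On the server, BeginPlay finds the manager and binds raw OSC messages, parsing `/beyond/cue/2/` live-control position addresses into per-joint X and Y arrays.
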(event OnSceneActivate(ReembodiedMachineOscHandler)
  (params (SceneIndex :type Integer) (PhaseIndex :type Integer))
  (Development|PrintText (Utilities|Text|FormatText "[Scene Index: {SceneIndex} StageIndex: {PhaseIndex}]" SceneIndex PhaseIndex) true true "(R=0.000000,G=1.000000,B=0.040489,A=1.000000)" 5.0)
  (CallFunction|HandleNewScenePhaseActivation SceneIndex PhaseIndex))

(event Custom|OnOscMessageReceived_Event
  (params (Message :type OSC%20Message%20Structure%20%28by%20ref%29) (IPAddress :type String) (Port :type Integer))
  (bind _returnvalue (Class|OSCManager|GetOSCMessageAddress Message))
  (bind _returnvalue_2 (Class|OSCManager|GetOSCAddressFullPath _returnvalue))
  (bind _value (Class|OSCManager|GetFloat Message))
  (Utilities|FlowControl|Sequence
    (:then_0
      (if (Utilities|Enum|Equal(Enum) (.RightS (Utilities|String|Split (.RightS (Utilities|String|Split (.RightS (Utilities|String|Split _returnvalue_2 "/beyond/cue/2/")) "/")) "livecontrol/pos" "IgnoreCase" "FromEnd")) "x")
        (Utilities|Array|SetArrayElem (Variables|Default|GetJointsX) (Math|Conversions|ToInteger(Byte) (.LeftS (Utilities|String|Split (.RightS (Utilities|String|Split _returnvalue_2 "/beyond/cue/2/")) "/"))) _value true)))
    (:then_1
      (if (Utilities|Enum|Equal(Enum) (.RightS (Utilities|String|Split (.RightS (Utilities|String|Split (.RightS (Utilities|String|Split _returnvalue_2 "/beyond/cue/2/")) "/")) "livecontrol/pos" "IgnoreCase" "FromEnd")) "y")
        (Utilities|Array|SetArrayElem (Variables|Default|GetJointsY) (Math|Conversions|ToInteger(Byte) (.LeftS (Utilities|String|Split (.RightS (Utilities|String|Split _returnvalue_2 "/beyond/cue/2/")) "/"))) _value true)))
    (:then_2
      (Variables|Default|SetJointNumber (.LeftS (Utilities|String|Split (.RightS (Utilities|String|Split _returnvalue_2 "/beyond/cue/2/")) "/")))
      (Variables|Default|SetJointAxis (.RightS (Utilities|String|Split (.RightS (Utilities|String|Split (.RightS (Utilities|String|Split _returnvalue_2 "/beyond/cue/2/")) "/")) "livecontrol/pos" "IgnoreCase" "FromEnd"))))))

(event EventBeginPlay
  (if (Networking|IsServer)
    (Utilities|FlowControl|Sequence
      (:then_1
        (EventDispatchers|AssignOnOscMessageReceived (Variables|/Script/PremiereLaserShow.ReembodiedMachineOscHandler|GetOscServer (Variables|Default|GetReembodiedMachineOscHandler)) (delegate Custom|OnOscMessageReceived_Event))
        (bind _returnvalue (Actor|GetActorOfClass "/PremierLaserShow/Blueprints/BP_PremierSequenceManager.BP_PremierSequenceManager_C"))
        (Utilities|IsValid _returnvalue
          (:Is%20Valid
            (Variables|Default|SetSequenceManager _returnvalue))
          (:Is%20Not%20Valid
            (Development|PrintString "BP_PremiereSequenceMangaer not in Scene. 
Please make sure it's in the scene." true true "(R=1.000000,G=0.002721,B=0.000000,A=1.000000)" 15.0)
            (Actor|Tick|SetActorTickEnabled false)))))
    (else
      (Actor|Tick|SetActorTickEnabled false))))

(fn ConstructionScript)

(fn HandleNewScenePhaseActivation
  (params (SceneIndex :type Integer) (PhaseIndex :type Integer))
  (bind _sequencemanager (Variables|Default|GetSequenceManager))
  (bind _sequencemanager_2 (Variables|Default|GetSequenceManager))
  (bind _sequencemanager_3 (Variables|Default|GetSequenceManager))
  (bind _sequencemanager_4 (Variables|Default|GetSequenceManager))
  (bind _sequencemanager_5 (Variables|Default|GetSequenceManager))
  (bind _sequencemanager_6 (Variables|Default|GetSequenceManager))
  (bind _sequencemanager_7 (Variables|Default|GetSequenceManager))
  (Default|CallOnNewScenePhaseActivation SceneIndex PhaseIndex)
  (Utilities|FlowControl|Sequence
    (:then_0
      (Utilities|IsValid (Variables|Default|GetSequenceManager)
        (:Is%20Not%20Valid
          (Development|PrintString "BP_PremiereSequenceMangaer not in Scene. 
Please make sure it's in the scene." true true "(R=1.000000,G=0.002721,B=0.000000,A=1.000000)" 15.0)
          (return))))
    (:then_1
      (if (== SceneIndex 1)
        (switch int PhaseIndex
          (:Default
            (CallFunction|LogScenePhaseActivationError SceneIndex PhaseIndex)
            (return))
          (:0
            (Variables|/PremierLaserShow/Blueprints/BP_PremierSequenceManager.BP_PremierSequenceManager_C|SetStage1-End _sequencemanager_3 true)
            (Variables|/PremierLaserShow/Blueprints/BP_PremierSequenceManager.BP_PremierSequenceManager_C|SetStage1-Start _sequencemanager_3 false)
            (return))
          (:1
            (Variables|/PremierLaserShow/Blueprints/BP_PremierSequenceManager.BP_PremierSequenceManager_C|SetStage1-End (Variables|Default|GetSequenceManager) false)
            (Variables|/PremierLaserShow/Blueprints/BP_PremierSequenceManager.BP_PremierSequenceManager_C|SetStage1-Start (Variables|Default|GetSequenceManager) true)
            (return))
          (:2
            (Variables|/PremierLaserShow/Blueprints/BP_PremierSequenceManager.BP_PremierSequenceManager_C|SetStage1-MultiLights (Variables|Default|GetSequenceManager) true)
            (return))
          (:3
            (Variables|/PremierLaserShow/Blueprints/BP_PremierSequenceManager.BP_PremierSequenceManager_C|SetStage1-SwitchToLHand (Variables|Default|GetSequenceManager) true)
            (return))
          (:4
            (Variables|/PremierLaserShow/Blueprints/BP_PremierSequenceManager.BP_PremierSequenceManager_C|SetStage1-SwitchToRHand (Variables|Default|GetSequenceManager) true)
            (return))
          (:5
            (Variables|/PremierLaserShow/Blueprints/BP_PremierSequenceManager.BP_PremierSequenceManager_C|SetStage1-SwitchToRFoot (Variables|Default|GetSequenceManager) true)
            (return))
          (:6
            (Variables|/PremierLaserShow/Blueprints/BP_PremierSequenceManager.BP_PremierSequenceManager_C|SetStage1-RandomBones (Variables|Default|GetSequenceManager) true)
            (return))
          (:7
            (Variables|/PremierLaserShow/Blueprints/BP_PremierSequenceManager.BP_PremierSequenceManager_C|SetStage1-MultiRandomBones (Variables|Default|GetSequenceManager) true)
            (return)))))
    (:then_2
      (if (== SceneIndex 2)
        (switch int PhaseIndex
          (:Default
            (CallFunction|LogScenePhaseActivationError SceneIndex PhaseIndex)
            (return))
          (:0
            (Variables|/PremierLaserShow/Blueprints/BP_PremierSequenceManager.BP_PremierSequenceManager_C|SetStage2-End _sequencemanager_5 true)
            (Variables|/PremierLaserShow/Blueprints/BP_PremierSequenceManager.BP_PremierSequenceManager_C|SetStage2-Start _sequencemanager_5 false)
            (return))
          (:1
            (Variables|/PremierLaserShow/Blueprints/BP_PremierSequenceManager.BP_PremierSequenceManager_C|SetStage2-Start (Variables|Default|GetSequenceManager) true)
            (return))
          (:2
            (Variables|/PremierLaserShow/Blueprints/BP_PremierSequenceManager.BP_PremierSequenceManager_C|SetStage2-StartLaser (Variables|Default|GetSequenceManager) true)
            (return))
          (:3
            (Variables|/PremierLaserShow/Blueprints/BP_PremierSequenceManager.BP_PremierSequenceManager_C|SetStage2-LightsBreathe (Variables|Default|GetSequenceManager) true)
            (return))
          (:4
            (Variables|/PremierLaserShow/Blueprints/BP_PremierSequenceManager.BP_PremierSequenceManager_C|SetStage2-FadeOutSpotlights (Variables|Default|GetSequenceManager) true)
            (return))
          (:5
            (Variables|/PremierLaserShow/Blueprints/BP_PremierSequenceManager.BP_PremierSequenceManager_C|SetStage2-LaserExtend (Variables|Default|GetSequenceManager) true)
            (Variables|Default|SetStage2/5Triggered true)
            (return))
          (:6
            (if (Variables|Default|GetStage2/5Triggered)
              (Variables|/PremierLaserShow/Blueprints/BP_PremierSequenceManager.BP_PremierSequenceManager_C|SetStage2-SwitchToDancer (Variables|Default|GetSequenceManager) true)
              (return))))))
    (:then_3
      (if (== SceneIndex 3)
        (switch int PhaseIndex
          (:Default
            (CallFunction|LogScenePhaseActivationError SceneIndex PhaseIndex)
            (return))
          (:0
            (Variables|/PremierLaserShow/Blueprints/BP_PremierSequenceManager.BP_PremierSequenceManager_C|SetStage3-Start _sequencemanager_6 false)
            (Variables|/PremierLaserShow/Blueprints/BP_PremierSequenceManager.BP_PremierSequenceManager_C|SetStage3-Full _sequencemanager_6 false)
            (return))
          (:1
            (Variables|/PremierLaserShow/Blueprints/BP_PremierSequenceManager.BP_PremierSequenceManager_C|SetStage3-Start (Variables|Default|GetSequenceManager) true)
            (return))
          (:2
            (Variables|/PremierLaserShow/Blueprints/BP_PremierSequenceManager.BP_PremierSequenceManager_C|SetStage3-Full (Variables|Default|GetSequenceManager) true)
            (return)))))
    (:then_4
      (if (== SceneIndex 4)
        (switch int PhaseIndex
          (:Default
            (CallFunction|LogScenePhaseActivationError SceneIndex PhaseIndex)
            (return))
          (:1
            (Variables|/PremierLaserShow/Blueprints/BP_PremierSequenceManager.BP_PremierSequenceManager_C|SetStage4-StartSpotlight1 (Variables|Default|GetSequenceManager) true)
            (return))
          (:2
            (Variables|/PremierLaserShow/Blueprints/BP_PremierSequenceManager.BP_PremierSequenceManager_C|SetStage4-StartSpotlight2 (Variables|Default|GetSequenceManager) true)
            (return))
          (:3
            (Variables|/PremierLaserShow/Blueprints/BP_PremierSequenceManager.BP_PremierSequenceManager_C|SetStage4-StartSpotlight3 (Variables|Default|GetSequenceManager) true)
            (return))
          (:4
            (Variables|/PremierLaserShow/Blueprints/BP_PremierSequenceManager.BP_PremierSequenceManager_C|SetStage4-StartSpotlight4 (Variables|Default|GetSequenceManager) true)
            (return))
          (:5
            (Variables|/PremierLaserShow/Blueprints/BP_PremierSequenceManager.BP_PremierSequenceManager_C|SetStage4-StartSpotlight5 (Variables|Default|GetSequenceManager) true)
            (return))
          (:6
            (Variables|/PremierLaserShow/Blueprints/BP_PremierSequenceManager.BP_PremierSequenceManager_C|SetStage4-StartSpotlight6 (Variables|Default|GetSequenceManager) true)
            (return))
          (:7
            (Variables|/PremierLaserShow/Blueprints/BP_PremierSequenceManager.BP_PremierSequenceManager_C|SetStage4-StartSpotlight7 (Variables|Default|GetSequenceManager) true)
            (return))
          (:8
            (Variables|/PremierLaserShow/Blueprints/BP_PremierSequenceManager.BP_PremierSequenceManager_C|SetStage4-StartSpotlight8 (Variables|Default|GetSequenceManager) true)
            (return))
          (:9
            (Variables|/PremierLaserShow/Blueprints/BP_PremierSequenceManager.BP_PremierSequenceManager_C|SetStage4-StopAll (Variables|Default|GetSequenceManager) true)
            (return)))))
    (:then_5
      (if (== SceneIndex 5)
        (switch int PhaseIndex
          (:Default
            (CallFunction|LogScenePhaseActivationError SceneIndex PhaseIndex)
            (return))
          (:0
            (Variables|/PremierLaserShow/Blueprints/BP_PremierSequenceManager.BP_PremierSequenceManager_C|SetStage5-Start _sequencemanager false)
            (Variables|/PremierLaserShow/Blueprints/BP_PremierSequenceManager.BP_PremierSequenceManager_C|SetStage5-EndSequence _sequencemanager true)
            (return))
          (:1
            (Variables|/PremierLaserShow/Blueprints/BP_PremierSequenceManager.BP_PremierSequenceManager_C|SetStage5-Start (Variables|Default|GetSequenceManager) true)
            (return))
          (:2
            (Variables|/PremierLaserShow/Blueprints/BP_PremierSequenceManager.BP_PremierSequenceManager_C|SetStage5-HeadControl (Variables|Default|GetSequenceManager) true)
            (return)))))
    (:then_6
      (if (== SceneIndex 6)
        (switch int PhaseIndex
          (:Default
            (CallFunction|LogScenePhaseActivationError SceneIndex PhaseIndex)
            (return))
          (:0
            (Variables|/PremierLaserShow/Blueprints/BP_PremierSequenceManager.BP_PremierSequenceManager_C|SetStage6-End _sequencemanager_4 true)
            (Variables|/PremierLaserShow/Blueprints/BP_PremierSequenceManager.BP_PremierSequenceManager_C|SetStage6-Start _sequencemanager_4 false)
            (Variables|/PremierLaserShow/Blueprints/BP_PremierSequenceManager.BP_PremierSequenceManager_C|SetStage6-SplitLaserTime _sequencemanager_4 false)
            (return))
          (:1
            (Variables|/PremierLaserShow/Blueprints/BP_PremierSequenceManager.BP_PremierSequenceManager_C|SetStage6-Start (Variables|Default|GetSequenceManager) true)
            (Variables|/PremierLaserShow/Blueprints/BP_PremierSequenceManager.BP_PremierSequenceManager_C|SetStage6-End (Variables|Default|GetSequenceManager) false)
            (return))
          (:2
            (Variables|/PremierLaserShow/Blueprints/BP_PremierSequenceManager.BP_PremierSequenceManager_C|SetStage6-CompleteCircle (Variables|Default|GetSequenceManager) true)
            (Variables|/PremierLaserShow/Blueprints/BP_PremierSequenceManager.BP_PremierSequenceManager_C|SetStage6-End (Variables|Default|GetSequenceManager) false)
            (return))
          (:3
            (Variables|/PremierLaserShow/Blueprints/BP_PremierSequenceManager.BP_PremierSequenceManager_C|SetStage6-ArmsInfluenceCircle (Variables|Default|GetSequenceManager) true)
            (return))
          (:4
            (Variables|/PremierLaserShow/Blueprints/BP_PremierSequenceManager.BP_PremierSequenceManager_C|SetStage6-ArmsNoInfluence (Variables|Default|GetSequenceManager) true)
            (return))
          (:5
            (Variables|/PremierLaserShow/Blueprints/BP_PremierSequenceManager.BP_PremierSequenceManager_C|SetStage6-SplitLaserTime (Variables|Default|GetSequenceManager) true)
            (return))
          (:6
            (Variables|/PremierLaserShow/Blueprints/BP_PremierSequenceManager.BP_PremierSequenceManager_C|SetStage6-SpotlightsOn (Variables|Default|GetSequenceManager) true)
            (return)))))
    (:then_7
      (if (== SceneIndex 7)
        (switch int PhaseIndex
          (:Default
            (CallFunction|LogScenePhaseActivationError SceneIndex PhaseIndex))
          (:0
            (Variables|/PremierLaserShow/Blueprints/BP_PremierSequenceManager.BP_PremierSequenceManager_C|SetStage7-End5 (Variables|Default|GetSequenceManager) true)
            (Variables|/PremierLaserShow/Blueprints/BP_PremierSequenceManager.BP_PremierSequenceManager_C|SetStage7-Start (Variables|Default|GetSequenceManager) false))
          (:1
            (Variables|/PremierLaserShow/Blueprints/BP_PremierSequenceManager.BP_PremierSequenceManager_C|SetStage7-Start (Variables|Default|GetSequenceManager) true))
          (:2
            (Variables|/PremierLaserShow/Blueprints/BP_PremierSequenceManager.BP_PremierSequenceManager_C|SetStage7-Exaggerated (Variables|Default|GetSequenceManager) true))
          (:3
            (Variables|/PremierLaserShow/Blueprints/BP_PremierSequenceManager.BP_PremierSequenceManager_C|SetStage7-Calm (Variables|Default|GetSequenceManager) true))
          (:4
            (Variables|/PremierLaserShow/Blueprints/BP_PremierSequenceManager.BP_PremierSequenceManager_C|SetStage7-Jiggles (Variables|Default|GetSequenceManager) true))
          (:5
            (Variables|/PremierLaserShow/Blueprints/BP_PremierSequenceManager.BP_PremierSequenceManager_C|SetStage7-Calm2 (Variables|Default|GetSequenceManager) true))
          (:6
            (Variables|/PremierLaserShow/Blueprints/BP_PremierSequenceManager.BP_PremierSequenceManager_C|SetStage7-End1 (Variables|Default|GetSequenceManager) true))
          (:7
            (Variables|/PremierLaserShow/Blueprints/BP_PremierSequenceManager.BP_PremierSequenceManager_C|SetStage7-End2 (Variables|Default|GetSequenceManager) true))
          (:8
            (Variables|/PremierLaserShow/Blueprints/BP_PremierSequenceManager.BP_PremierSequenceManager_C|SetStage7-End3 (Variables|Default|GetSequenceManager) true))
          (:9
            (Variables|/PremierLaserShow/Blueprints/BP_PremierSequenceManager.BP_PremierSequenceManager_C|SetStage7-End4 (Variables|Default|GetSequenceManager) true)))))
    (:then_8
      (if (== SceneIndex 8)
        (switch int PhaseIndex
          (:Default
            (CallFunction|LogScenePhaseActivationError SceneIndex PhaseIndex)
            (return))
          (:0
            (Variables|/PremierLaserShow/Blueprints/BP_PremierSequenceManager.BP_PremierSequenceManager_C|SetStage8-Start _sequencemanager_7 false)
            (Variables|/PremierLaserShow/Blueprints/BP_PremierSequenceManager.BP_PremierSequenceManager_C|SetStage8-LaserDance _sequencemanager_7 false)
            (Variables|/PremierLaserShow/Blueprints/BP_PremierSequenceManager.BP_PremierSequenceManager_C|SetStage8-FadeOut _sequencemanager_7 true)
            (return))
          (:1
            (Variables|/PremierLaserShow/Blueprints/BP_PremierSequenceManager.BP_PremierSequenceManager_C|SetStage8-Start (Variables|Default|GetSequenceManager) true)
            (return))
          (:2
            (Variables|/PremierLaserShow/Blueprints/BP_PremierSequenceManager.BP_PremierSequenceManager_C|SetStage8-LaserDance (Variables|Default|GetSequenceManager) true)
            (return)))))
    (:then_9
      (if (== SceneIndex 9)
        (switch int PhaseIndex
          (:Default
            (CallFunction|LogScenePhaseActivationError SceneIndex PhaseIndex)
            (return))
          (:0
            (Variables|/PremierLaserShow/Blueprints/BP_PremierSequenceManager.BP_PremierSequenceManager_C|SetStage9-Start _sequencemanager_2 false)
            (Variables|/PremierLaserShow/Blueprints/BP_PremierSequenceManager.BP_PremierSequenceManager_C|SetStage9-Maze1 _sequencemanager_2 false)
            (Variables|/PremierLaserShow/Blueprints/BP_PremierSequenceManager.BP_PremierSequenceManager_C|SetStage9-Maze2 _sequencemanager_2 false)
            (Variables|/PremierLaserShow/Blueprints/BP_PremierSequenceManager.BP_PremierSequenceManager_C|SetStage9-Maze3 _sequencemanager_2 false)
            (Variables|/PremierLaserShow/Blueprints/BP_PremierSequenceManager.BP_PremierSequenceManager_C|SetStage9-FinalSequence _sequencemanager_2 true)
            (return))
          (:1
            (Variables|/PremierLaserShow/Blueprints/BP_PremierSequenceManager.BP_PremierSequenceManager_C|SetStage9-Start (Variables|Default|GetSequenceManager) true)
            (return))
          (:2
            (Variables|/PremierLaserShow/Blueprints/BP_PremierSequenceManager.BP_PremierSequenceManager_C|SetStage9-Maze1 (Variables|Default|GetSequenceManager) true)
            (return))
          (:3
            (Variables|/PremierLaserShow/Blueprints/BP_PremierSequenceManager.BP_PremierSequenceManager_C|SetStage9-Maze2 (Variables|Default|GetSequenceManager) true)
            (return))
          (:4
            (Variables|/PremierLaserShow/Blueprints/BP_PremierSequenceManager.BP_PremierSequenceManager_C|SetStage9-Maze3 (Variables|Default|GetSequenceManager) true)
            (return))
          (:5
            (Variables|/PremierLaserShow/Blueprints/BP_PremierSequenceManager.BP_PremierSequenceManager_C|SetStage9-Maze4 (Variables|Default|GetSequenceManager) true)
            (return)))))
    (:then_10
      (if (== SceneIndex 10)
        (switch int PhaseIndex
          (:Default
            (CallFunction|LogScenePhaseActivationError SceneIndex PhaseIndex))
          (:0
            (Variables|/PremierLaserShow/Blueprints/BP_PremierSequenceManager.BP_PremierSequenceManager_C|SetStage10-FadeGroup2 (Variables|Default|GetSequenceManager) true))
          (:1
            (Variables|/PremierLaserShow/Blueprints/BP_PremierSequenceManager.BP_PremierSequenceManager_C|SetStage10-Start (Variables|Default|GetSequenceManager) true))
          (:2
            (Variables|/PremierLaserShow/Blueprints/BP_PremierSequenceManager.BP_PremierSequenceManager_C|SetStage10-FadeGroup1 (Variables|Default|GetSequenceManager) true)))))
    (:then_11
      (if (== SceneIndex 11)
        (switch int PhaseIndex
          (:Default
            (CallFunction|LogScenePhaseActivationError SceneIndex PhaseIndex))
          (:0
            (Variables|/PremierLaserShow/Blueprints/BP_PremierSequenceManager.BP_PremierSequenceManager_C|SetRestart (Variables|Default|GetSequenceManager) true)))))))

(fn LogScenePhaseActivationError
  (params (SceneIndex :type Integer) (PhaseIndex :type Integer))
  (Development|PrintText (Utilities|Text|FormatText "No such scene-phase combination. 
Scene Index {SceneIndex} Phase Index {PhaseIndex}" SceneIndex PhaseIndex) true true "(R=1.000000,G=0.000000,B=0.000000,A=1.000000)" 15.0))