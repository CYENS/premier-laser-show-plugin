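; Example Blueprint that shows data from its ReembodiedMachineOscHandler as on-screen debug text.
; Handler events print scene and phase changes in green, and loop over received light pan, tilt, intensity, offset, joint association and laser line arrays.
; Each array element prints with an index-based key, so its message updates in place instead of stacking.
; Joint associations reuse the intensity key suffix, so those two readouts collide at matching indices.
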(event OnLightJointAssociationReceived(ReembodiedMachineOscHandler)
  (params (LightJointAssociation :type Array%20of%20Integers))
  (for (_array_element _array_index) LightJointAssociation
    (Development|PrintText (Utilities|Text|FormatText "Join Association {LightJointIndex}: {AssociatedJoint}" _array_index _array_element) true true "(R=0.000000,G=0.660000,B=1.000000,A=1.000000)" 2.0 (Utilities|String|StringToName (Utilities|String|ToString(Text) (Utilities|Text|FormatText "{LightJointIndex}_Intensity" _array_index))))))

(event OnLightOffsetsReceived(ReembodiedMachineOscHandler)
  (params (Offsets :type Array%20of%20Vector%202f%20Structures))
  (for (_array_element _array_index) Offsets
    (Development|PrintText (Utilities|Text|FormatText "Offset {OffsetIndex}: ({X}, {Y})" _array_index (.X (Math|Vector2D|BreakVector2D _array_element)) (.Y (Math|Vector2D|BreakVector2D _array_element))) true true "(R=0.000000,G=0.660000,B=1.000000,A=1.000000)" 2.0 (Utilities|String|StringToName (Utilities|String|ToString(Text) (Utilities|Text|FormatText "{OffsetIndex}_Offset" _array_index))))))

(event OnLaserLinesReceived(ReembodiedMachineOscHandler)
  (params (LineData :type Array%20of%20Vector%204f%20Structures))
  (for (_array_element _array_index) LineData
    (Development|PrintText (Utilities|Text|FormatText "Line {LineIndex}: ({X}, {Y}, {Angle}, {Length})" _array_index (.X (Math|Vector4|BreakVector4 _array_element)) (.Y (Math|Vector4|BreakVector4 _array_element)) (.Z (Math|Vector4|BreakVector4 _array_element)) (.W (Math|Vector4|BreakVector4 _array_element))) true true "(R=0.000000,G=0.660000,B=1.000000,A=1.000000)" 2.0 (Utilities|String|StringToName (Utilities|String|ToString(Text) (Utilities|Text|FormatText "{LineIndex}_Line" _array_index))))))

(event OnSceneActivate(ReembodiedMachineOscHandler)
  (params (SceneIndex :type Integer) (PhaseIndex :type Integer))
  (Development|PrintText (Utilities|Text|FormatText "[Scene Index: {SceneIndex} StageIndex: {PhaseIndex}]" SceneIndex PhaseIndex) true true "(R=0.000000,G=1.000000,B=0.040489,A=1.000000)" 5.0))

(event OnLightTiltsReceived(ReembodiedMachineOscHandler)
  (params (TiltValues :type Array%20of%20Vector%202f%20Structures))
  (for (_array_element _array_index) TiltValues
    (Development|PrintText (Utilities|Text|FormatText "Tilt {TiltIndex}: ({X}, {Y})" _array_index (.X (Math|Vector2D|BreakVector2D _array_element)) (.Y (Math|Vector2D|BreakVector2D _array_element))) true true "(R=0.000000,G=0.660000,B=1.000000,A=1.000000)" 2.0 (Utilities|String|StringToName (Utilities|String|ToString(Text) (Utilities|Text|FormatText "{TiltIndex}_Tilt" _array_index))))))

(event OnLightIntensitiesReceived(ReembodiedMachineOscHandler)
  (params (Intensities :type Array%20of%20Floats%20%28single-precision%29))
  (for (_array_element _array_index) Intensities
    (Development|PrintText (Utilities|Text|FormatText "Intensity {IntensityIndex}: {Intensity}" _array_index _array_element) true true "(R=0.000000,G=0.660000,B=1.000000,A=1.000000)" 2.0 (Utilities|String|StringToName (Utilities|String|ToString(Text) (Utilities|Text|FormatText "{IntensityIndex}_Intensity" _array_index))))))

(event OnLightPansReceived(ReembodiedMachineOscHandler)
  (params (PanValues :type Array%20of%20Vector%202f%20Structures))
  (for (_array_element _array_index) PanValues
    (Development|PrintText (Utilities|Text|FormatText "Pan {PanIndex}: ({X}, {Y})" _array_index (.X (Math|Vector2D|BreakVector2D _array_element)) (.Y (Math|Vector2D|BreakVector2D _array_element))) true true "(R=0.000000,G=0.660000,B=1.000000,A=1.000000)" 2.0 (Utilities|String|StringToName (Utilities|String|ToString(Text) (Utilities|Text|FormatText "{PanIndex}_Pan" _array_index))))))

(fn ConstructionScript)