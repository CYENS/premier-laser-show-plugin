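; Dancer actor that samples world-space bone transforms from its DancerSkeleton for arms, hands, upper spine, legs and toes.
; Each Tick sets global time dilation from TimeMultiplier, stores each transform and updates a lagged position after DelayTime.
; Velocities are the offset from that lagged position multiplied, not divided, by DeltaSeconds.
; Getters expose transforms and some delayed positions and velocities; the construction script pre-fills only arm and hand transforms.
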(event EventTick
  (params (DeltaSeconds :type Float%20%28single-precision%29))
  (Variables|Time|SetDelta%20Seconds DeltaSeconds)
  (Utilities|Time|SetGlobalTimeDilation (Variables|Time|GetTimeMultiplier))
  (Utilities|FlowControl|Sequence
    (:then_0
      (bind _output_get (Variables|LArm|SetLArmTransform (Transformation|GetBoneTransform (Variables|Default|GetDancerSkeleton) "LeftArm" "RTS_World")))
      (Utilities|FlowControl|Sequence
        (:then_0
          (Variables|LArm|SetLArmVelocity (* (- (.location _output_get) (stale _output_get_2)) (Variables|Time|GetDelta%20Seconds))))
        (:then_1
          (Utilities|FlowControl|Delay (Variables|Time|GetDelayTime))
          (bind _output_get_2 (Variables|LArm|SetLArmDelayPos (.location _output_get))))))
    (:then_1
      (bind _output_get_3 (Variables|LForeArm|SetLForeArmTransform (Transformation|GetBoneTransform (Variables|Default|GetDancerSkeleton) "LeftForeArm" "RTS_World")))
      (Utilities|FlowControl|Sequence
        (:then_0
          (Variables|LForeArm|SetLForeArmVelocity (* (- (.location _output_get_3) (stale _output_get_4)) (Variables|Time|GetDelta%20Seconds))))
        (:then_1
          (Utilities|FlowControl|Delay (Variables|Time|GetDelayTime))
          (bind _output_get_4 (Variables|LForeArm|SetLForeArmDelayPos (.location _output_get_3))))))
    (:then_2
      (bind _output_get_5 (Variables|LHand|SetLHandTransform (Transformation|GetBoneTransform (Variables|Default|GetDancerSkeleton) "LeftHand" "RTS_World")))
      (Utilities|FlowControl|Sequence
        (:then_0
          (Variables|LHand|SetLHandVelocity (* (- (.location _output_get_5) (stale _output_get_6)) (Variables|Time|GetDelta%20Seconds))))
        (:then_1
          (Utilities|FlowControl|Delay (Variables|Time|GetDelayTime))
          (bind _output_get_6 (Variables|LHand|SetLHandDelayPos (.location _output_get_5))))))
    (:then_3
      (bind _output_get_7 (Variables|RArm|SetRArmTransform (Transformation|GetBoneTransform (Variables|Default|GetDancerSkeleton) "RightArm" "RTS_World")))
      (Utilities|FlowControl|Sequence
        (:then_0
          (Variables|RArm|SetRArmVelocity (* (- (.location _output_get_7) (stale _output_get_8)) (Variables|Time|GetDelta%20Seconds))))
        (:then_1
          (Utilities|FlowControl|Delay (Variables|Time|GetDelayTime))
          (bind _output_get_8 (Variables|RArm|SetRArmDelayPos (.location _output_get_7))))))
    (:then_4
      (bind _output_get_9 (Variables|RForeArm|SetRForeArmTransform (Transformation|GetBoneTransform (Variables|Default|GetDancerSkeleton) "RightForeArm" "RTS_World")))
      (Utilities|FlowControl|Sequence
        (:then_0
          (Variables|RForeArm|SetRForeArmVelocity (* (- (.location _output_get_9) (stale _output_get_10)) (Variables|Time|GetDelta%20Seconds))))
        (:then_1
          (Utilities|FlowControl|Delay (Variables|Time|GetDelayTime))
          (bind _output_get_10 (Variables|RForeArm|SetRForeArmDelayPos (.location _output_get_9))))))
    (:then_5
      (bind _output_get_11 (Variables|RHand|SetRHandTransform (Transformation|GetBoneTransform (Variables|Default|GetDancerSkeleton) "RightHand" "RTS_World")))
      (Utilities|FlowControl|Sequence
        (:then_0
          (Variables|RHand|SetRHandVelocity (* (- (.location _output_get_11) (stale _output_get_12)) (Variables|Time|GetDelta%20Seconds))))
        (:then_1
          (Utilities|FlowControl|Delay (Variables|Time|GetDelayTime))
          (bind _output_get_12 (Variables|RHand|SetRHandDelayPos (.location _output_get_11))))))
    (:then_6
      (bind _output_get_13 (Variables|Spine|SetUpperSpineTransform (Transformation|GetBoneTransform (Variables|Default|GetDancerSkeleton) "Spine2" "RTS_World")))
      (Utilities|FlowControl|Sequence
        (:then_0
          (Variables|Spine|SetSpineVelocity (* (- (.location _output_get_13) (stale _output_get_14)) (Variables|Time|GetDelta%20Seconds))))
        (:then_1
          (Utilities|FlowControl|Delay (Variables|Time|GetDelayTime))
          (bind _output_get_14 (Variables|Spine|SetSpineDelayPos (.location _output_get_13))))))
    (:then_7
      (bind _output_get_15 (Variables|RLeg|SetRLegTransform (Transformation|GetBoneTransform (Variables|Default|GetDancerSkeleton) "RightLeg" "RTS_World")))
      (Utilities|FlowControl|Sequence
        (:then_0
          (Variables|RLeg|SetRLegVelocity (* (- (.location _output_get_15) (stale _output_get_16)) (Variables|Time|GetDelta%20Seconds))))
        (:then_1
          (Utilities|FlowControl|Delay (Variables|Time|GetDelayTime))
          (bind _output_get_16 (Variables|RLeg|SetRLegDelayPos (.location _output_get_15))))))
    (:then_8
      (bind _output_get_17 (Variables|LLeg|SetLLegTransform (Transformation|GetBoneTransform (Variables|Default|GetDancerSkeleton) "LeftLeg" "RTS_World")))
      (Utilities|FlowControl|Sequence
        (:then_0
          (Variables|LLeg|SetLLegVelocity (* (- (.location _output_get_17) (stale _output_get_18)) (Variables|Time|GetDelta%20Seconds))))
        (:then_1
          (Utilities|FlowControl|Delay (Variables|Time|GetDelayTime))
          (bind _output_get_18 (Variables|LLeg|SetLLegDelayPos (.location _output_get_17))))))
    (:then_9
      (bind _output_get_19 (Variables|RToe|SetRToeTransform (Transformation|GetBoneTransform (Variables|Default|GetDancerSkeleton) "RightToeBase" "RTS_World")))
      (Utilities|FlowControl|Sequence
        (:then_0
          (Variables|RToe|SetRToeVelocity (* (- (.location _output_get_19) (stale _output_get_20)) (Variables|Time|GetDelta%20Seconds))))
        (:then_1
          (Utilities|FlowControl|Delay (Variables|Time|GetDelayTime))
          (bind _output_get_20 (Variables|RToe|SetRToeDelayPos (.location _output_get_19))))))
    (:then_10
      (bind _output_get_21 (Variables|LToe|SetLToeTransform (Transformation|GetBoneTransform (Variables|Default|GetDancerSkeleton) "LeftToeBase" "RTS_World")))
      (Utilities|FlowControl|Sequence
        (:then_0
          (Variables|LToe|SetLToeVelocity (* (- (.location _output_get_21) (stale _output_get_22)) (Variables|Time|GetDelta%20Seconds))))
        (:then_1
          (Utilities|FlowControl|Delay (Variables|Time|GetDelayTime))
          (bind _output_get_22 (Variables|LToe|SetLToeDelayPos (.location _output_get_21))))))))

(fn ConstructionScript
  (Utilities|FlowControl|Sequence
    (:then_0
      (Variables|LArm|SetLArmTransform (Transformation|GetBoneTransform (Variables|Default|GetDancerSkeleton) "LeftArm" "RTS_World")))
    (:then_1
      (Variables|LForeArm|SetLForeArmTransform (Transformation|GetBoneTransform (Variables|Default|GetDancerSkeleton) "LeftForeArm" "RTS_World")))
    (:then_2
      (Variables|LHand|SetLHandTransform (Transformation|GetBoneTransform (Variables|Default|GetDancerSkeleton) "LeftHand" "RTS_World")))
    (:then_3
      (Variables|RArm|SetRArmTransform (Transformation|GetBoneTransform (Variables|Default|GetDancerSkeleton) "RightArm" "RTS_World")))
    (:then_4
      (Variables|RForeArm|SetRForeArmTransform (Transformation|GetBoneTransform (Variables|Default|GetDancerSkeleton) "RightForeArm" "RTS_World")))
    (:then_5
      (Variables|RHand|SetRHandTransform (Transformation|GetBoneTransform (Variables|Default|GetDancerSkeleton) "RightHand" "RTS_World")))))

(fn GetLArmDelayPos
  (return (Variables|LArm|GetLArmDelayPos)))

(fn GetLArmTransform
  (return (Variables|LArm|GetLArmTransform)))

(fn GetLArmVelocity
  (return (Variables|LArm|GetLArmVelocity)))

(fn GetLForeArmTransform
  (return (Variables|LForeArm|GetLForeArmTransform)))

(fn GetLForeArmVelocity
  (return (Variables|LForeArm|GetLForeArmVelocity)))

(fn GetLHandDelayPos
  (return (Variables|LHand|GetLHandDelayPos)))

(fn GetLHandTransform
  (return (Variables|LHand|GetLHandTransform)))

(fn GetLHandVelocity
  (return (Variables|LHand|GetLHandVelocity)))

(fn GetLLegDelayPos
  (return (Variables|LLeg|GetLLegDelayPos)))

(fn GetLLegTransform
  (return (Variables|LLeg|GetLLegTransform)))

(fn GetLToeDelayPos
  (return (Variables|LToe|GetLToeDelayPos)))

(fn GetLToeTransform
  (return (Variables|LToe|GetLToeTransform)))

(fn GetRArmDelayPos
  (return (Variables|RArm|GetRArmDelayPos)))

(fn GetRArmTransform
  (return (Variables|RArm|GetRArmTransform)))

(fn GetRArmVelocity
  (return (Variables|RArm|GetRArmVelocity)))

(fn GetRForeArmTransform
  (return (Variables|RForeArm|GetRForeArmTransform)))

(fn GetRForeArmVelocity
  (return (Variables|RForeArm|GetRForeArmVelocity)))

(fn GetRHandDelayPos
  (return (Variables|RHand|GetRHandDelayPos)))

(fn GetRHandTransform
  (return (Variables|RHand|GetRHandTransform)))

(fn GetRHandVelocity
  (return (Variables|RHand|GetRHandVelocity)))

(fn GetRLegDelayPos
  (return (Variables|RLeg|GetRLegDelayPos)))

(fn GetRLegTransform
  (return (Variables|RLeg|GetRLegTransform)))

(fn GetRToeDelayPos
  (return (Variables|RToe|GetRToeDelayPos)))

(fn GetRToeTransform
  (return (Variables|RToe|GetRToeTransform)))

(fn GetSpineDelayPos
  (return (Variables|Spine|GetSpineDelayPos)))

(fn GetUpperSpineTransform
  (return (Variables|Spine|GetUpperSpineTransform)))