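; Laser rig actor whose six beams track the arm, forearm and hand bones on both sides of BP_Dancer, at runtime and from the construction script.
; A shared macro aims each beam with a sine drift scaled by bone velocity, line-traces past the target, stretches the mesh to the hit and moves its area light there.
; Tick drives a shared dynamic material and the lights' intensity and colour, collapsing beams and zeroing lights when tracking is off.
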(event EventBeginPlay
  (bind _outactors (Actor|GetAllActorswithTag "Structure"))
  (Variables|Default|SetStructureActors _outactors)
  (bind _returnvalue (Actor|GetActorOfClass "/PremierLaserShow/BP_Dancer.BP_Dancer_C"))
  (Variables|Default|SetDancerRef _returnvalue)
  (bind _returnvalue_2 (Rendering|Material|CreateDynamicMaterialInstance (Rendering|Material|GetMaterial (Variables|Default|GetLaser3) 0) "None" "None" :!class /Script/Engine.KismetMaterialLibrary))
  (Variables|Default|SetLaserMaterial _returnvalue_2)
  (Rendering|Material|SetMaterial (Variables|Default|GetLaser1) 0 (Variables|Default|GetLaserMaterial)))

(event EventTick
  (params (DeltaSeconds :type Float%20%28single-precision%29))
  (bind _lasermaterialintensity (Variables|Default|GetLaserMaterialIntensity))
  (bind _laser1 (Variables|Default|GetLaser1))
  (bind _laser1arealight (Variables|Default|GetLaser1AreaLight))
  (bind _laser1arealight_2 (Variables|Default|GetLaser1AreaLight))
  (bind _lasermaterial (Variables|Default|GetLaserMaterial))
  (bind _returnvalue (Transformation|GetWorldScale _laser1))
  (bind _output_get (Variables|Default|SetDelta%20Seconds DeltaSeconds))
  (Variables|Default|SetTime (+ _output_get (Variables|Default|GetTime)))
  (Utilities|FlowControl|Sequence
    (:then_0
      (if (Variables|Default|GetIsTracking)
        (Utilities|FlowControl|Sequence
          (:then_0
            (Utilities|LinetraceTrackerMacro (Variables|Default|GetLaser4) (.location (Variables|/PremierLaserShow/BP_Dancer.BP_Dancer_C|GetLArmTransform (Variables|Default|GetDancerRef))) (Variables|Default|GetLaser4AreaLight) (Math|Integer|Absolute(Integer) 0)))
          (:then_1
            (Utilities|LinetraceTrackerMacro (Variables|Default|GetLaser5) (.location (Variables|/PremierLaserShow/BP_Dancer.BP_Dancer_C|GetLForeArmTransform (Variables|Default|GetDancerRef))) (Variables|Default|GetLaser5AreaLight) (Math|Integer|Absolute(Integer) 1)))
          (:then_2
            (Utilities|LinetraceTrackerMacro (Variables|Default|GetLaser6) (.location (Variables|/PremierLaserShow/BP_Dancer.BP_Dancer_C|GetLHandTransform (Variables|Default|GetDancerRef))) (Variables|Default|GetLaser6AreaLight) (Math|Integer|Absolute(Integer) 2)))
          (:then_3
            (Utilities|LinetraceTrackerMacro (Variables|Default|GetLaser3) (.location (Variables|/PremierLaserShow/BP_Dancer.BP_Dancer_C|GetRArmTransform (Variables|Default|GetDancerRef))) (Variables|Default|GetLaser3AreaLight) (Math|Integer|Absolute(Integer) 3)))
          (:then_4
            (Utilities|LinetraceTrackerMacro (Variables|Default|GetLaser2) (.location (Variables|/PremierLaserShow/BP_Dancer.BP_Dancer_C|GetRForeArmTransform (Variables|Default|GetDancerRef))) (Variables|Default|GetLaser2AreaLight) (Math|Integer|Absolute(Integer) 4)))
          (:then_5
            (Utilities|LinetraceTrackerMacro (Variables|Default|GetLaser1) (.location (Variables|/PremierLaserShow/BP_Dancer.BP_Dancer_C|GetRHandTransform (Variables|Default|GetDancerRef))) (Variables|Default|GetLaser1AreaLight) (Math|Integer|Absolute(Integer) 5)))
          (:then_6
            (Utilities|IsValid (Variables|Default|GetLaserMaterial)
              (:Is%20Valid
                (Rendering|Material|SetScalarParameterValue _lasermaterial "BrightnessMultiplier" (Variables|Default|GetLaserMaterialIntensity) :!class /Script/Engine.MaterialInstanceDynamic)
                (Rendering|Material|SetVectorParameterValue _lasermaterial "Colour" (Variables|Default|GetLaserMaterialColour) :!class /Script/Engine.MaterialInstanceDynamic)
                (Rendering|Material|SetScalarParameterValue _lasermaterial "SpiralOpacity" (* _lasermaterialintensity 0.1) :!class /Script/Engine.MaterialInstanceDynamic)
                (Rendering|Material|SetScalarParameterValue _lasermaterial "BrightnessMultiplier" _lasermaterialintensity :!class /Script/Engine.MaterialInstanceDynamic)
                (Rendering|Material|SetScalarParameterValue _lasermaterial "SpiralIntensity1" (* _lasermaterialintensity 5.0) :!class /Script/Engine.MaterialInstanceDynamic)
                (Rendering|Material|SetScalarParameterValue _lasermaterial "SpiralIntensity2" (* _lasermaterialintensity 3.0) :!class /Script/Engine.MaterialInstanceDynamic)
                (if (Variables|Default|GetMultiplyLaserIntensity)
                  (Rendering|Components|Light|SetIntensity (Variables|Default|GetLaser1AreaLight) (* (Variables|Default|GetLaserAreaIntensity) (* (Variables|Default|GetLaserMaterialIntensity) (Variables|Default|GetLaserMaterialMultiplier))))
                  (else
                    (Rendering|Components|Light|SetIntensity _laser1arealight_2 (Variables|Default|GetLaserAreaIntensity))))
                (Rendering|Components|Light|SetLightColor _laser1arealight_2 (Variables|Default|GetAreaLightColour) true)))))
        (else
          (Transformation|SetWorldRotation _laser1 (Math|Rotator|MakeRotator 0.0 0.0 0.0) false false)
          (Transformation|SetWorldScale3D _laser1 (Math|Vector|MakeVector (.x _returnvalue) (.y _returnvalue) 0.0))
          (Transformation|SetWorldLocation _laser1arealight (Transformation|GetWorldLocation (Variables|Default|GetLightRigParent)) false false)
          (Rendering|Components|Light|SetIntensity _laser1arealight 0.0))))
    (:then_1
      (Utilities|Array|SetArrayElem (Variables|Default|GetBoneVelocities) 0 (Math|Vector|VectorLength (Variables|/PremierLaserShow/BP_Dancer.BP_Dancer_C|GetLArmVelocity (Variables|Default|GetDancerRef))))
      (Utilities|Array|SetArrayElem (Variables|Default|GetBoneVelocities) 1 (Math|Vector|VectorLength (Variables|/PremierLaserShow/BP_Dancer.BP_Dancer_C|GetLForeArmVelocity (Variables|Default|GetDancerRef))))
      (Utilities|Array|SetArrayElem (Variables|Default|GetBoneVelocities) 2 (Math|Vector|VectorLength (Variables|/PremierLaserShow/BP_Dancer.BP_Dancer_C|GetLHandVelocity (Variables|Default|GetDancerRef))))
      (Utilities|Array|SetArrayElem (Variables|Default|GetBoneVelocities) 3 (Math|Vector|VectorLength (Variables|/PremierLaserShow/BP_Dancer.BP_Dancer_C|GetRArmVelocity (Variables|Default|GetDancerRef))))
      (Utilities|Array|SetArrayElem (Variables|Default|GetBoneVelocities) 4 (Math|Vector|VectorLength (Variables|/PremierLaserShow/BP_Dancer.BP_Dancer_C|GetRForeArmVelocity (Variables|Default|GetDancerRef))))
      (Utilities|Array|SetArrayElem (Variables|Default|GetBoneVelocities) 5 (Math|Vector|VectorLength (Variables|/PremierLaserShow/BP_Dancer.BP_Dancer_C|GetRHandVelocity (Variables|Default|GetDancerRef))))
      (for (_array_element _array_index) (Variables|Default|GetBoneVelocities)
        (Utilities|Array|SetArrayElem (Variables|Default|GetOffsetDrifts) _array_index (* (* _array_element (Math|Trig|Sin(Radians) (Variables|Default|GetTime))) (Variables|Default|GetAngleVariance)))))))

(fn ConstructionScript
  (bind _laser1arealight (Variables|Default|GetLaser1AreaLight))
  (bind _perlinnoisearray (Variables|Default|GetPerlinNoiseArray))
  (bind _lasermaterial (Variables|Default|GetLaserMaterial))
  (Utilities|Array|Clear _perlinnoisearray)
  (Utilities|FlowControl|Sequence
    (:then_0
      (bind _outactors (Actor|GetAllActorswithTag "Structure"))
      (Variables|Default|SetStructureActors _outactors)
      (bind _returnvalue (Actor|GetActorOfClass "/PremierLaserShow/BP_Dancer.BP_Dancer_C"))
      (Variables|Default|SetDancerRef _returnvalue)
      (if (Variables|Default|GetIsTracking)
        (Utilities|FlowControl|Sequence
          (:then_0
            (Utilities|LinetraceTrackerMacro (Variables|Default|GetLaser4) (.location (Variables|/PremierLaserShow/BP_Dancer.BP_Dancer_C|GetLArmTransform (Variables|Default|GetDancerRef))) (Variables|Default|GetLaser4AreaLight) (Math|Integer|Absolute(Integer) 0)))
          (:then_1
            (Utilities|LinetraceTrackerMacro (Variables|Default|GetLaser5) (.location (Variables|/PremierLaserShow/BP_Dancer.BP_Dancer_C|GetLForeArmTransform (Variables|Default|GetDancerRef))) (Variables|Default|GetLaser5AreaLight) (Math|Integer|Absolute(Integer) 1)))
          (:then_2
            (Utilities|LinetraceTrackerMacro (Variables|Default|GetLaser6) (.location (Variables|/PremierLaserShow/BP_Dancer.BP_Dancer_C|GetLHandTransform (Variables|Default|GetDancerRef))) (Variables|Default|GetLaser6AreaLight) (Math|Integer|Absolute(Integer) 2)))
          (:then_3
            (Utilities|LinetraceTrackerMacro (Variables|Default|GetLaser3) (.location (Variables|/PremierLaserShow/BP_Dancer.BP_Dancer_C|GetRArmTransform (Variables|Default|GetDancerRef))) (Variables|Default|GetLaser3AreaLight) (Math|Integer|Absolute(Integer) 3)))
          (:then_4
            (Utilities|LinetraceTrackerMacro (Variables|Default|GetLaser2) (.location (Variables|/PremierLaserShow/BP_Dancer.BP_Dancer_C|GetRForeArmTransform (Variables|Default|GetDancerRef))) (Variables|Default|GetLaser2AreaLight) (Math|Integer|Absolute(Integer) 4)))
          (:then_5
            (Utilities|LinetraceTrackerMacro (Variables|Default|GetLaser1) (.location (Variables|/PremierLaserShow/BP_Dancer.BP_Dancer_C|GetRHandTransform (Variables|Default|GetDancerRef))) (Variables|Default|GetLaser1AreaLight) (Math|Integer|Absolute(Integer) 5)))
          (:then_6
            (Rendering|Material|SetScalarParameterValue _lasermaterial "BrightnessMultiplier" (Variables|Default|GetLaserMaterialIntensity) :!class /Script/Engine.MaterialInstanceDynamic)
            (Rendering|Material|SetVectorParameterValue _lasermaterial "Colour" (Variables|Default|GetLaserMaterialColour) :!class /Script/Engine.MaterialInstanceDynamic)
            (if (Variables|Default|GetMultiplyLaserIntensity)
              (Rendering|Components|Light|SetIntensity (Variables|Default|GetLaser1AreaLight) (* (Variables|Default|GetLaserAreaIntensity) (* (Variables|Default|GetLaserMaterialIntensity) (Variables|Default|GetLaserMaterialMultiplier))))
              (else
                (Rendering|Components|Light|SetIntensity _laser1arealight (Variables|Default|GetLaserAreaIntensity))))
            (Rendering|Components|Light|SetLightColor _laser1arealight (Variables|Default|GetAreaLightColour) true)))))
    (:then_1
      (Utilities|Array|AddUnique _perlinnoisearray (Math|Random|RandomFloatinRange 0.0 1e+02))
      (Utilities|Array|AddUnique _perlinnoisearray (Math|Random|RandomFloatinRange 0.0 1e+02))
      (Utilities|Array|AddUnique _perlinnoisearray (Math|Random|RandomFloatinRange 0.0 1e+02))
      (Utilities|Array|AddUnique _perlinnoisearray (Math|Random|RandomFloatinRange 0.0 1e+02))
      (Utilities|Array|AddUnique _perlinnoisearray (Math|Random|RandomFloatinRange 0.0 1e+02))
      (Utilities|Array|AddUnique _perlinnoisearray (Math|Random|RandomFloatinRange 0.0 1e+02)))))