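; OSC handler test Blueprint that drives staged show sequences and streams Stage 10 data.
; Scene activation events map scene and phase indices to stage flags on BP_PremierSequenceManager, printing errors for unmatched branches.
; Every received OSC message is read as groups of four floats, scaled into Stage10Struct position, length and rotation, with debug prints.
; Tick copies these into Stage10AllValues, adding a position-negated mirror at index offset 16.
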(event OnSceneActivate(ReembodiedMachineOscHandler)
  (params (SceneIndex :type Integer) (PhaseIndex :type Integer))
  (Development|PrintText (Utilities|Text|FormatText "[Scene Index: {SceneIndex} StageIndex: {PhaseIndex}]" SceneIndex PhaseIndex) true true "(R=0.000000,G=1.000000,B=0.040489,A=1.000000)" 5.0)
  (CallFunction|HandleNewScenePhaseActivation SceneIndex PhaseIndex))

(event Custom|OnOscMessageReceived_Event
  (params (Message :type OSC%20Message%20Structure%20%28by%20ref%29) (IPAddress :type String) (Port :type Integer))
  (bind _stage10struct (Variables|Default|GetStage10Struct))
  (Utilities|FlowControl|Sequence
    (:then_0
      (bind _returnvalue (Class|OSCManager|GetOSCMessageAddress Message))
      (bind _returnvalue_2 (Class|OSCManager|GetOSCAddressFullPath _returnvalue))
      (Development|PrintString _returnvalue_2 true true "(R=0.000000,G=0.660000,B=1.000000,A=1.000000)" 2.0 "Address"))
    (:then_1
      (bind _values (Class|OSCManager|GetAllFloats Message))
      (bind _output_get (Variables|Default|SetValues _values))
      (for (_ _array_index) _stage10struct
        (Utilities|Array|SetArrayElem _stage10struct _array_index (Utilities|Struct|MakeStage10_Struct (/ (Utilities|Array|Get(acopy) _output_get (* _array_index 4)) 1e+02) (/ (Utilities|Array|Get(acopy) _output_get (+ (* _array_index 4) 1)) 1e+02) (/ (Utilities|Array|Get(acopy) _output_get (+ (+ (+ (* _array_index 4) 1) 1) 1)) 1e+03) (Utilities|Array|Get(acopy) _output_get (+ (+ (* _array_index 4) 1) 1))) true)
        (Development|PrintString (Utilities|String|ToString(Float) (Utilities|Array|Get(acopy) _output_get (* _array_index 4))) true true "(R=0.000000,G=0.660000,B=1.000000,A=1.000000)" 2.0 "1")
        (Development|PrintString (Utilities|String|ToString(Float) (Utilities|Array|Get(acopy) _output_get (+ (* _array_index 4) 1))) true true "(R=0.000000,G=1.000000,B=0.205075,A=1.000000)" 2.0 "2")
        (Development|PrintString (Utilities|String|ToString(Float) (Utilities|Array|Get(acopy) _output_get (+ (+ (* _array_index 4) 1) 1))) true true "(R=1.000000,G=0.264812,B=0.000000,A=1.000000)" 2.0 "3")
        (Development|PrintString (Utilities|String|ToString(Float) (Utilities|Array|Get(acopy) _output_get (+ (+ (+ (* _array_index 4) 1) 1) 1))) true true "(R=1.000000,G=0.000000,B=0.922396,A=1.000000)" 2.0 "4")))))

(event EventBeginPlay
  (Utilities|FlowControl|Sequence
    (:then_1
      (EventDispatchers|AssignOnOscMessageReceived (Variables|/Script/PremiereLaserShow.ReembodiedMachineOscHandler|GetOscServer (Variables|Default|GetReembodiedMachineOscHandler)) (delegate Custom|OnOscMessageReceived_Event))
      (bind _returnvalue (Actor|GetActorOfClass "/PremierLaserShow/Blueprints/BP_PremierSequenceManager.BP_PremierSequenceManager_C"))
      (Utilities|IsValid _returnvalue
        (:Is%20Valid
          (Variables|Default|SetSequenceManager _returnvalue))
        (:Is%20Not%20Valid
          (Development|PrintString "BP_PremiereSequenceMangaer not in Scene. 
Please make sure it's in the scene." true true "(R=1.000000,G=0.002721,B=0.000000,A=1.000000)" 15.0)
          (Actor|Tick|SetActorTickEnabled false))))))

(event EventTick
  (params (DeltaSeconds :type Float%20%28single-precision%29))
  (bind _stage10allvalues (Variables|Default|GetStage10AllValues))
  (for (_array_element _array_index) (Variables|Default|GetStage10Struct)
    (Utilities|Array|SetArrayElem _stage10allvalues _array_index (Utilities|Struct|MakeStage10_Struct (.xposition _array_element) (.yposition _array_element) (.length _array_element) (.rotation _array_element)) true)
    (Utilities|Array|SetArrayElem _stage10allvalues (+ _array_index 16) (Utilities|Struct|MakeStage10_Struct (* (.xposition _array_element) -1.0) (* (.yposition _array_element) -1.0) (.length _array_element) (.rotation _array_element)) true)))

(fn ConstructionScript)

(fn HandleNewScenePhaseActivation
  (params (SceneIndex :type Integer) (PhaseIndex :type Integer))
  (bind _sequencemanager (Variables|Default|GetSequenceManager))
  (bind _sequencemanager_2 (Variables|Default|GetSequenceManager))
  (bind _sequencemanager_3 (Variables|Default|GetSequenceManager))
  (bind _sequencemanager_4 (Variables|Default|GetSequenceManager))
  (bind _sequencemanager_5 (Variables|Default|GetSequenceManager))
  (bind _sequencemanager_6 (Variables|Default|GetSequenceManager))
  (Utilities|FlowControl|Sequence
    (:then_0
      (Utilities|IsValid (Variables|Default|GetSequenceManager)
        (:Is%20Not%20Valid
          (Development|PrintString "BP_PremiereSequenceMangaer not in Scene. 
Please make sure it's in the scene." true true "(R=1.000000,G=0.002721,B=0.000000,A=1.000000)" 15.0)
          (return))))
    (:then_1
      (if (== SceneIndex 1)
        (switch int PhaseIndex
          (:Default
            (CallFunction|LogScenePhaseActivationError SceneIndex PhaseIndex)
            (return))
          (:0
            (Variables|/PremierLaserShow/Blueprints/BP_PremierSequenceManager.BP_PremierSequenceManager_C|SetStage1-End _sequencemanager_3 true)
            (Variables|/PremierLaserShow/Blueprints/BP_PremierSequenceManager.BP_PremierSequenceManager_C|SetStage1-Start _sequencemanager_3 false)
            (return))
          (:1
            (Variables|/PremierLaserShow/Blueprints/BP_PremierSequenceManager.BP_PremierSequenceManager_C|SetStage1-End (Variables|Default|GetSequenceManager) false)
            (Variables|/PremierLaserShow/Blueprints/BP_PremierSequenceManager.BP_PremierSequenceManager_C|SetStage1-Start (Variables|Default|GetSequenceManager) true)
            (return))
          (:2
            (Variables|/PremierLaserShow/Blueprints/BP_PremierSequenceManager.BP_PremierSequenceManager_C|SetStage1-MultiLights (Variables|Default|GetSequenceManager) true)
            (return))
          (:3
            (Variables|/PremierLaserShow/Blueprints/BP_PremierSequenceManager.BP_PremierSequenceManager_C|SetStage1-SwitchToLHand (Variables|Default|GetSequenceManager) true)
            (return))
          (:4
            (Variables|/PremierLaserShow/Blueprints/BP_PremierSequenceManager.BP_PremierSequenceManager_C|SetStage1-SwitchToRHand (Variables|Default|GetSequenceManager) true)
            (return))
          (:5
            (Variables|/PremierLaserShow/Blueprints/BP_PremierSequenceManager.BP_PremierSequenceManager_C|SetStage1-SwitchToRFoot (Variables|Default|GetSequenceManager) true)
            (return))
          (:6
            (Variables|/PremierLaserShow/Blueprints/BP_PremierSequenceManager.BP_PremierSequenceManager_C|SetStage1-RandomBones (Variables|Default|GetSequenceManager) true)
            (return))
          (:7
            (Variables|/PremierLaserShow/Blueprints/BP_PremierSequenceManager.BP_PremierSequenceManager_C|SetStage1-MultiRandomBones (Variables|Default|GetSequenceManager) true)
            (return)))
        (else
          (CallFunction|LogScenePhaseActivationError SceneIndex PhaseIndex))))
    (:then_2
      (if (== SceneIndex 2)
        (switch int PhaseIndex
          (:Default
            (CallFunction|LogScenePhaseActivationError SceneIndex PhaseIndex)
            (return))
          (:0
            (Variables|/PremierLaserShow/Blueprints/BP_PremierSequenceManager.BP_PremierSequenceManager_C|SetStage2-End _sequencemanager_5 true)
            (Variables|/PremierLaserShow/Blueprints/BP_PremierSequenceManager.BP_PremierSequenceManager_C|SetStage2-Start _sequencemanager_5 false)
            (return))
          (:1
            (Variables|/PremierLaserShow/Blueprints/BP_PremierSequenceManager.BP_PremierSequenceManager_C|SetStage2-Start (Variables|Default|GetSequenceManager) true)
            (return))
          (:2
            (Variables|/PremierLaserShow/Blueprints/BP_PremierSequenceManager.BP_PremierSequenceManager_C|SetStage2-SwitchToDancer (Variables|Default|GetSequenceManager) true)
            (return)))
        (else
          (CallFunction|LogScenePhaseActivationError SceneIndex PhaseIndex))))
    (:then_3
      (if (== SceneIndex 3)
        (switch int PhaseIndex
          (:Default
            (CallFunction|LogScenePhaseActivationError SceneIndex PhaseIndex)
            (return))
          (:0
            (Variables|/PremierLaserShow/Blueprints/BP_PremierSequenceManager.BP_PremierSequenceManager_C|SetStage3-Start _sequencemanager_6 false)
            (Variables|/PremierLaserShow/Blueprints/BP_PremierSequenceManager.BP_PremierSequenceManager_C|SetStage3-Full _sequencemanager_6 false)
            (return))
          (:1
            (Variables|/PremierLaserShow/Blueprints/BP_PremierSequenceManager.BP_PremierSequenceManager_C|SetStage3-Start (Variables|Default|GetSequenceManager) true)
            (return))
          (:2
            (Variables|/PremierLaserShow/Blueprints/BP_PremierSequenceManager.BP_PremierSequenceManager_C|SetStage3-Full (Variables|Default|GetSequenceManager) true)
            (return)))
        (else
          (CallFunction|LogScenePhaseActivationError SceneIndex PhaseIndex))))
    (:then_4
      (if (== SceneIndex 4)
        (switch int PhaseIndex
          (:Default
            (CallFunction|LogScenePhaseActivationError SceneIndex PhaseIndex)
            (return))
          (:0
            (Variables|/PremierLaserShow/Blueprints/BP_PremierSequenceManager.BP_PremierSequenceManager_C|SetStage4-Start (Variables|Default|GetSequenceManager) false)
            (return))
          (:1
            (Variables|/PremierLaserShow/Blueprints/BP_PremierSequenceManager.BP_PremierSequenceManager_C|SetStage4-Start (Variables|Default|GetSequenceManager) true)
            (return)))
        (else
          (CallFunction|LogScenePhaseActivationError SceneIndex PhaseIndex))))
    (:then_6
      (if (== SceneIndex 6)
        (switch int PhaseIndex
          (:Default
            (CallFunction|LogScenePhaseActivationError SceneIndex PhaseIndex)
            (return))
          (:0
            (Variables|/PremierLaserShow/Blueprints/BP_PremierSequenceManager.BP_PremierSequenceManager_C|SetStage6-End _sequencemanager_4 true)
            (Variables|/PremierLaserShow/Blueprints/BP_PremierSequenceManager.BP_PremierSequenceManager_C|SetStage6-Start _sequencemanager_4 false)
            (Variables|/PremierLaserShow/Blueprints/BP_PremierSequenceManager.BP_PremierSequenceManager_C|SetStage6-SplitLaserTime _sequencemanager_4 false)
            (return))
          (:1
            (Variables|/PremierLaserShow/Blueprints/BP_PremierSequenceManager.BP_PremierSequenceManager_C|SetStage6-Start (Variables|Default|GetSequenceManager) true)
            (Variables|/PremierLaserShow/Blueprints/BP_PremierSequenceManager.BP_PremierSequenceManager_C|SetStage6-End (Variables|Default|GetSequenceManager) false)
            (return))
          (:2
            (Variables|/PremierLaserShow/Blueprints/BP_PremierSequenceManager.BP_PremierSequenceManager_C|SetStage6-ArmsInfluenceCircle (Variables|Default|GetSequenceManager) true)
            (return))
          (:3
            (Variables|/PremierLaserShow/Blueprints/BP_PremierSequenceManager.BP_PremierSequenceManager_C|SetStage6-SplitLaserTime (Variables|Default|GetSequenceManager) true)
            (return)))
        (else
          (CallFunction|LogScenePhaseActivationError SceneIndex PhaseIndex))))
    (:then_8
      (if (== SceneIndex 8)
        (switch int PhaseIndex
          (:Default
            (CallFunction|LogScenePhaseActivationError SceneIndex PhaseIndex)
            (return))
          (:0
            (Variables|/PremierLaserShow/Blueprints/BP_PremierSequenceManager.BP_PremierSequenceManager_C|SetStage8-Start _sequencemanager false)
            (Variables|/PremierLaserShow/Blueprints/BP_PremierSequenceManager.BP_PremierSequenceManager_C|SetStage8-LaserDance _sequencemanager false)
            (Variables|/PremierLaserShow/Blueprints/BP_PremierSequenceManager.BP_PremierSequenceManager_C|SetStage8-FadeOut _sequencemanager false)
            (return))
          (:1
            (Variables|/PremierLaserShow/Blueprints/BP_PremierSequenceManager.BP_PremierSequenceManager_C|SetStage8-Start (Variables|Default|GetSequenceManager) true)
            (return))
          (:2
            (Variables|/PremierLaserShow/Blueprints/BP_PremierSequenceManager.BP_PremierSequenceManager_C|SetStage8-LaserDance (Variables|Default|GetSequenceManager) true)
            (return))
          (:3
            (Variables|/PremierLaserShow/Blueprints/BP_PremierSequenceManager.BP_PremierSequenceManager_C|SetStage8-FadeOut (Variables|Default|GetSequenceManager) true)
            (return)))
        (else
          (CallFunction|LogScenePhaseActivationError SceneIndex PhaseIndex))))
    (:then_9
      (if (== SceneIndex 9)
        (switch int PhaseIndex
          (:Default
            (CallFunction|LogScenePhaseActivationError SceneIndex PhaseIndex))
          (:0
            (Variables|/PremierLaserShow/Blueprints/BP_PremierSequenceManager.BP_PremierSequenceManager_C|SetStage9-Start _sequencemanager_2 false)
            (Variables|/PremierLaserShow/Blueprints/BP_PremierSequenceManager.BP_PremierSequenceManager_C|SetStage9-Maze1 _sequencemanager_2 false)
            (Variables|/PremierLaserShow/Blueprints/BP_PremierSequenceManager.BP_PremierSequenceManager_C|SetStage9-Maze2 _sequencemanager_2 false)
            (Variables|/PremierLaserShow/Blueprints/BP_PremierSequenceManager.BP_PremierSequenceManager_C|SetStage9-Maze3 _sequencemanager_2 false)
            (Variables|/PremierLaserShow/Blueprints/BP_PremierSequenceManager.BP_PremierSequenceManager_C|SetStage9-FinalSequence _sequencemanager_2 false)
            (return))
          (:1
            (Variables|/PremierLaserShow/Blueprints/BP_PremierSequenceManager.BP_PremierSequenceManager_C|SetStage9-Start (Variables|Default|GetSequenceManager) true)
            (return))
          (:2
            (Variables|/PremierLaserShow/Blueprints/BP_PremierSequenceManager.BP_PremierSequenceManager_C|SetStage9-Maze1 (Variables|Default|GetSequenceManager) true)
            (return))
          (:3
            (Variables|/PremierLaserShow/Blueprints/BP_PremierSequenceManager.BP_PremierSequenceManager_C|SetStage9-Maze2 (Variables|Default|GetSequenceManager) true)
            (return))
          (:4
            (Variables|/PremierLaserShow/Blueprints/BP_PremierSequenceManager.BP_PremierSequenceManager_C|SetStage9-Maze3 (Variables|Default|GetSequenceManager) true)
            (return))
          (:5
            (Variables|/PremierLaserShow/Blueprints/BP_PremierSequenceManager.BP_PremierSequenceManager_C|SetStage9-FinalSequence (Variables|Default|GetSequenceManager) true)
            (return)))
        (else
          (CallFunction|LogScenePhaseActivationError SceneIndex PhaseIndex))))))

(fn LogScenePhaseActivationError
  (params (SceneIndex :type Integer) (PhaseIndex :type Integer))
  (Development|PrintText (Utilities|Text|FormatText "No such scene-phase combination. 
Scene Index {SceneIndex} Phase Index {PhaseIndex}" SceneIndex PhaseIndex) true true "(R=1.000000,G=0.000000,B=0.000000,A=1.000000)" 15.0))