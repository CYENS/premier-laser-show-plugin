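; Dancer actor that tracks arm, forearm and hand motion on both sides of its skeleton, plus the upper spine transform.
; Construction caches the limb transforms; Tick refreshes them and applies TimeMultiplier as global time dilation.
; Each limb's velocity is its offset from a position stored after a Delay, multiplied (not divided) by DeltaSeconds, so it is not true velocity.
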(event EventTick
  (params (DeltaSeconds :type Float%20%28single-precision%29))
  (Variables|Default|SetDelta%20Seconds DeltaSeconds)
  (Utilities|Time|SetGlobalTimeDilation (Variables|Default|GetTimeMultiplier))
  (Utilities|FlowControl|Sequence
    (:then_0
      (bind _output_get (Variables|Default|SetLArmTransform (Transformation|GetBoneTransform (Variables|Default|GetDancerSkeleton) "LeftArm" "RTS_World")))
      (Utilities|FlowControl|Sequence
        (:then_0
          (Variables|Default|SetLArmVelocity (* (- (.location _output_get) (stale _output_get_2)) (Variables|Default|GetDelta%20Seconds))))
        (:then_1
          (Utilities|FlowControl|Delay (Variables|Default|GetDelayTime))
          (bind _output_get_2 (Variables|Default|SetLArmDelayPos (.location _output_get))))))
    (:then_1
      (bind _output_get_3 (Variables|Default|SetLForeArmTransform (Transformation|GetBoneTransform (Variables|Default|GetDancerSkeleton) "LeftForeArm" "RTS_World")))
      (Utilities|FlowControl|Sequence
        (:then_0
          (Variables|Default|SetLForeArmVelocity (* (- (.location _output_get_3) (stale _output_get_4)) (Variables|Default|GetDelta%20Seconds))))
        (:then_1
          (Utilities|FlowControl|Delay (Variables|Default|GetDelayTime))
          (bind _output_get_4 (Variables|Default|SetLForeArmDelayPos (.location _output_get_3))))))
    (:then_2
      (bind _output_get_5 (Variables|Default|SetLHandTransform (Transformation|GetBoneTransform (Variables|Default|GetDancerSkeleton) "LeftHand" "RTS_World")))
      (Utilities|FlowControl|Sequence
        (:then_0
          (Variables|Default|SetLHandVelocity (* (- (.location _output_get_5) (stale _output_get_6)) (Variables|Default|GetDelta%20Seconds))))
        (:then_1
          (Utilities|FlowControl|Delay (Variables|Default|GetDelayTime))
          (bind _output_get_6 (Variables|Default|SetLHandDelayPos (.location _output_get_5))))))
    (:then_3
      (bind _output_get_7 (Variables|Default|SetRArmTransform (Transformation|GetBoneTransform (Variables|Default|GetDancerSkeleton) "RightArm" "RTS_World")))
      (Utilities|FlowControl|Sequence
        (:then_0
          (Variables|Default|SetRArmVelocity (* (- (.location _output_get_7) (stale _output_get_8)) (Variables|Default|GetDelta%20Seconds))))
        (:then_1
          (Utilities|FlowControl|Delay (Variables|Default|GetDelayTime))
          (bind _output_get_8 (Variables|Default|SetRArmDelayPos (.location _output_get_7))))))
    (:then_4
      (bind _output_get_9 (Variables|Default|SetRForeArmTransform (Transformation|GetBoneTransform (Variables|Default|GetDancerSkeleton) "RightForeArm" "RTS_World")))
      (Utilities|FlowControl|Sequence
        (:then_0
          (Variables|Default|SetRForeArmVelocity (* (- (.location _output_get_9) (stale _output_get_10)) (Variables|Default|GetDelta%20Seconds))))
        (:then_1
          (Utilities|FlowControl|Delay (Variables|Default|GetDelayTime))
          (bind _output_get_10 (Variables|Default|SetRForeArmDelayPos (.location _output_get_9))))))
    (:then_5
      (bind _output_get_11 (Variables|Default|SetRHandTransform (Transformation|GetBoneTransform (Variables|Default|GetDancerSkeleton) "RightHand" "RTS_World")))
      (Utilities|FlowControl|Sequence
        (:then_0
          (Variables|Default|SetRHandVelocity (* (- (.location _output_get_11) (stale _output_get_12)) (Variables|Default|GetDelta%20Seconds))))
        (:then_1
          (Utilities|FlowControl|Delay (Variables|Default|GetDelayTime))
          (bind _output_get_12 (Variables|Default|SetRHandDelayPos (.location _output_get_11))))))
    (:then_6
      (Variables|Default|SetUpperSpineTransform (Transformation|GetBoneTransform (Variables|Default|GetDancerSkeleton) "Spine2" "RTS_World")))))

(fn ConstructionScript
  (Utilities|FlowControl|Sequence
    (:then_0
      (Variables|Default|SetLArmTransform (Transformation|GetBoneTransform (Variables|Default|GetDancerSkeleton) "LeftArm" "RTS_World")))
    (:then_1
      (Variables|Default|SetLForeArmTransform (Transformation|GetBoneTransform (Variables|Default|GetDancerSkeleton) "LeftForeArm" "RTS_World")))
    (:then_2
      (Variables|Default|SetLHandTransform (Transformation|GetBoneTransform (Variables|Default|GetDancerSkeleton) "LeftHand" "RTS_World")))
    (:then_3
      (Variables|Default|SetRArmTransform (Transformation|GetBoneTransform (Variables|Default|GetDancerSkeleton) "RightArm" "RTS_World")))
    (:then_4
      (Variables|Default|SetRForeArmTransform (Transformation|GetBoneTransform (Variables|Default|GetDancerSkeleton) "RightForeArm" "RTS_World")))
    (:then_5
      (Variables|Default|SetRHandTransform (Transformation|GetBoneTransform (Variables|Default|GetDancerSkeleton) "RightHand" "RTS_World")))))