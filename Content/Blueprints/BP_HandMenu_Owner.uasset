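; Session owner's 3D hand menu, operated by overlaps from "Interactor"-tagged actors: public/private toggle, exit button and camera position arrows.
; The toggle updates every BP_HandMenu_Guest, exit requires a second touch during a countdown, and arrows cycle a wrapping camera index.
; Timelines animate meshes and dynamic-material brightness, with IsTransitioning blocking overlapping animations.
; Actions fire outward calls, though both toggle directions pass false; local handlers only print.
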(event OnComponentBeginOverlap(RightBox)
  (params (OverlappedComponent :type Primitive%20Component%20Object%20Reference) (OtherActor :type Actor%20Object%20Reference) (OtherComp :type Primitive%20Component%20Object%20Reference) (OtherBodyIndex :type Integer) (bFromSweep :type Boolean) (SweepResult :type Hit%20Result%20Structure%20%28by%20ref%29))
  (bind _arrowboxright (Variables|Default|GetArrowBoxRight))
  (bind _arrowboxright_2 (Variables|Default|GetArrowBoxRight))
  (bind _camera_currentnumber (Variables|Default|GetCamera-CurrentNumber))
  (bind _returnvalue (Transformation|GetRelativeTransform _arrowboxright))
  (bind _returnvalue_2 (Transformation|GetRelativeTransform _arrowboxright_2))
  (if (Actor|ActorHasTag OtherActor "Interactor")
    (if (not (Variables|Default|GetIsTransitioning))
      (Utilities|FlowControl|Sequence
        (:then_0
          (Variables|Default|SetIsTransitioning true)
          (bind _newtrack_0 (Timeline|RightCollidedStart PlayFromStart)
            (:Update
              (Transformation|SetRelativeLocation _arrowboxright (Math|Vector|Lerp(Vector) (Math|Vector|MakeVector (.x (.location _returnvalue)) (.y (.location _returnvalue)) (.z (.location _returnvalue))) (Math|Vector|MakeVector (.x (.location _returnvalue)) 6e+01 (.z (.location _returnvalue))) _newtrack_0) false false)
              (Rendering|Material|SetScalarParameterValue (Variables|Default|GetDynamicRightArrowMaterial) "Brightness" (Math|Float|Lerp 0.0 1.0 _newtrack_0) :!class /Script/Engine.MaterialInstanceDynamic)
              (Rendering|Material|SetScalarParameterValue (Variables|Default|GetDynamicCurrentCameraTextMaterial) "Brightness" (Math|Float|Lerp 0.0 1.0 _newtrack_0) :!class /Script/Engine.MaterialInstanceDynamic))
            (:Finished
              (bind _newtrack_0_2 (Timeline|RightCollidedEnd PlayFromStart)
                (:Update
                  (Transformation|SetRelativeLocation _arrowboxright_2 (Math|Vector|Lerp(Vector) (Math|Vector|MakeVector (.x (.location _returnvalue_2)) (.y (.location _returnvalue_2)) (.z (.location _returnvalue_2))) (Math|Vector|MakeVector (.x (.location _returnvalue_2)) -1e+02 (.z (.location _returnvalue_2))) _newtrack_0_2) false false)
                  (Rendering|Material|SetScalarParameterValue (Variables|Default|GetDynamicRightArrowMaterial) "Brightness" (Math|Float|Lerp 1.0 0.0 _newtrack_0_2) :!class /Script/Engine.MaterialInstanceDynamic)
                  (Rendering|Material|SetScalarParameterValue (Variables|Default|GetDynamicCurrentCameraTextMaterial) "Brightness" (Math|Float|Lerp 1.0 0.0 _newtrack_0_2) :!class /Script/Engine.MaterialInstanceDynamic))
                (:Finished
                  (Variables|Default|SetIsTransitioning false))))))
        (:then_1
          (if (>= (Variables|Default|GetCurrentCameraPositionIndex) (- (Variables|Default|GetNumberOfCameras) 1))
            (bind _output_get (Variables|Default|SetCurrentCameraPositionIndex 0))
            (Rendering|Components|TextRender|SetText _camera_currentnumber (Utilities|Text|ToText(Integer) (+ _output_get 1)))
            (else
              (bind _output_get_2 (Variables|Default|SetCurrentCameraPositionIndex (+ (Variables|Default|GetCurrentCameraPositionIndex) 1)))
              (Rendering|Components|TextRender|SetText _camera_currentnumber (Utilities|Text|ToText(Integer) (+ _output_get_2 1)))))
          (CallFunction|ChangeCamPosition (Variables|Default|GetCurrentCameraPositionIndex))
          (Default|CallCameraPositionChanged (Variables|Default|GetCurrentCameraPositionIndex)))))))

(event OnComponentBeginOverlap(Box)
  (params (OverlappedComponent :type Primitive%20Component%20Object%20Reference) (OtherActor :type Actor%20Object%20Reference) (OtherComp :type Primitive%20Component%20Object%20Reference) (OtherBodyIndex :type Integer) (bFromSweep :type Boolean) (SweepResult :type Hit%20Result%20Structure%20%28by%20ref%29))
  (bind _togglemesh (Variables|Default|GetToggleMesh))
  (bind _togglemesh_2 (Variables|Default|GetToggleMesh))
  (bind _returnvalue (Transformation|GetRelativeTransform _togglemesh))
  (bind _returnvalue_2 (Transformation|GetRelativeTransform _togglemesh_2))
  (if (Actor|ActorHasTag OtherActor "Interactor")
    (if (not (Variables|Default|GetIsTransitioning))
      (if (Variables|Default|GetIsPublic)
        (Utilities|FlowControl|Sequence
          (:then_0
            (Variables|Default|SetIsTransitioning true)
            (bind _newtrack_0 (Timeline|TransitionSessionToPrivate PlayFromStart)
              (:Update
                (Transformation|SetRelativeLocation _togglemesh (Math|Vector|Lerp(Vector) (Math|Vector|MakeVector (.x (.location _returnvalue)) (.y (.location _returnvalue)) (.z (.location _returnvalue))) (Math|Vector|MakeVector 3e+01 (.y (.location _returnvalue)) (.z (.location _returnvalue))) _newtrack_0) false false))
              (:Finished
                (Rendering|Components|TextRender|SetText (Variables|Default|GetSession-ToggleText) (Utilities|Text|ToText(String) "Private"))
                (Variables|Default|SetIsTransitioning false)
                (Variables|Default|SetIsPublic false)
                (bind _outactors (Actor|GetAllActorsOfClass "/PremierLaserShow/Blueprints/BP_HandMenu_Guest.BP_HandMenu_Guest_C"))
                (for _array_element _outactors
                  (Variables|/PremierLaserShow/Blueprints/BP_HandMenu_Guest.BP_HandMenu_Guest_C|SetIsPublic _array_element false)
                  (Default|SessionChanged _array_element)))))
          (:then_1
            (CallFunction|SessionPrivate))
          (:then_2
            (bind _newtrack_0_2 (Timeline|LightUpToggle PlayFromStart)
              (:Update
                (Rendering|Components|TextRender|SetText (Variables|Default|GetSession-ToggleText) (Utilities|Text|ToText(String) "Wait"))
                (Rendering|Material|SetScalarParameterValue (Variables|Default|GetDynamicToggleMaterial) "Brightness" (Math|Float|Lerp 0.0 1.0 _newtrack_0_2) :!class /Script/Engine.MaterialInstanceDynamic)
                (Rendering|Material|SetScalarParameterValue (Variables|Default|GetDynamicToggleTextMaterial) "Brightness" (Math|Float|Lerp 0.0 1.0 _newtrack_0_2) :!class /Script/Engine.MaterialInstanceDynamic))))
          (:then_3
            (Default|CallOnSessionPublicChange false)))
        (else
          (Utilities|FlowControl|Sequence
            (:then_0
              (Timeline|LightUpToggle PlayFromStart))
            (:then_1
              (Variables|Default|SetIsTransitioning true)
              (bind _newtrack_0_3 (Timeline|TransitionSessionToPublic PlayFromStart)
                (:Update
                  (Transformation|SetRelativeLocation _togglemesh_2 (Math|Vector|Lerp(Vector) (Math|Vector|MakeVector (.x (.location _returnvalue_2)) (.y (.location _returnvalue_2)) (.z (.location _returnvalue_2))) (Math|Vector|MakeVector 5.0 (.y (.location _returnvalue_2)) (.z (.location _returnvalue_2))) _newtrack_0_3) false false))
                (:Finished
                  (Rendering|Components|TextRender|SetText (Variables|Default|GetSession-ToggleText) (Utilities|Text|ToText(String) "Public"))
                  (Variables|Default|SetIsTransitioning false)
                  (Variables|Default|SetIsPublic true)
                  (bind _outactors_2 (Actor|GetAllActorsOfClass "/PremierLaserShow/Blueprints/BP_HandMenu_Guest.BP_HandMenu_Guest_C"))
                  (for _array_element_2 _outactors_2
                    (Variables|/PremierLaserShow/Blueprints/BP_HandMenu_Guest.BP_HandMenu_Guest_C|SetIsPublic _array_element_2 true)
                    (Default|SessionChanged _array_element_2)))))
            (:then_2
              (CallFunction|SessionPublic))
            (:then_3
              (Default|CallOnSessionPublicChange false))))))))

(event OnComponentBeginOverlap(LeftBox)
  (params (OverlappedComponent :type Primitive%20Component%20Object%20Reference) (OtherActor :type Actor%20Object%20Reference) (OtherComp :type Primitive%20Component%20Object%20Reference) (OtherBodyIndex :type Integer) (bFromSweep :type Boolean) (SweepResult :type Hit%20Result%20Structure%20%28by%20ref%29))
  (bind _arrowboxleft (Variables|Default|GetArrowBoxLeft))
  (bind _arrowboxleft_2 (Variables|Default|GetArrowBoxLeft))
  (bind _camera_currentnumber (Variables|Default|GetCamera-CurrentNumber))
  (bind _returnvalue (Transformation|GetRelativeTransform _arrowboxleft))
  (bind _returnvalue_2 (Transformation|GetRelativeTransform _arrowboxleft_2))
  (if (Actor|ActorHasTag OtherActor "Interactor")
    (if (not (Variables|Default|GetIsTransitioning))
      (Utilities|FlowControl|Sequence
        (:then_0
          (Variables|Default|SetIsTransitioning true)
          (bind _newtrack_0 (Timeline|LeftCollidedStart PlayFromStart)
            (:Update
              (Transformation|SetRelativeLocation _arrowboxleft_2 (Math|Vector|Lerp(Vector) (Math|Vector|MakeVector (.x (.location _returnvalue_2)) (.y (.location _returnvalue_2)) (.z (.location _returnvalue_2))) (Math|Vector|MakeVector (.x (.location _returnvalue_2)) 6e+01 (.z (.location _returnvalue_2))) _newtrack_0) false false)
              (Rendering|Material|SetScalarParameterValue (Variables|Default|GetDynamicLeftArrowMaterial) "Brightness" (Math|Float|Lerp 0.0 1.0 _newtrack_0) :!class /Script/Engine.MaterialInstanceDynamic)
              (Rendering|Material|SetScalarParameterValue (Variables|Default|GetDynamicCurrentCameraTextMaterial) "Brightness" (Math|Float|Lerp 0.0 1.0 _newtrack_0) :!class /Script/Engine.MaterialInstanceDynamic))
            (:Finished
              (bind _newtrack_0_2 (Timeline|LeftCollidedEnd PlayFromStart)
                (:Update
                  (Transformation|SetRelativeLocation _arrowboxleft (Math|Vector|Lerp(Vector) (Math|Vector|MakeVector (.x (.location _returnvalue)) (.y (.location _returnvalue)) (.z (.location _returnvalue))) (Math|Vector|MakeVector (.x (.location _returnvalue)) -1e+02 (.z (.location _returnvalue))) _newtrack_0_2) false false)
                  (Rendering|Material|SetScalarParameterValue (Variables|Default|GetDynamicLeftArrowMaterial) "Brightness" (Math|Float|Lerp 1.0 0.0 _newtrack_0_2) :!class /Script/Engine.MaterialInstanceDynamic)
                  (Rendering|Material|SetScalarParameterValue (Variables|Default|GetDynamicCurrentCameraTextMaterial) "Brightness" (Math|Float|Lerp 1.0 0.0 _newtrack_0_2) :!class /Script/Engine.MaterialInstanceDynamic))
                (:Finished
                  (Variables|Default|SetIsTransitioning false))))))
        (:then_1
          (if (<= (Variables|Default|GetCurrentCameraPositionIndex) 0)
            (bind _output_get (Variables|Default|SetCurrentCameraPositionIndex (- (Variables|Default|GetNumberOfCameras) 1)))
            (Rendering|Components|TextRender|SetText _camera_currentnumber (Utilities|Text|ToText(Integer) (+ _output_get 1)))
            (else
              (bind _output_get_2 (Variables|Default|SetCurrentCameraPositionIndex (- (Variables|Default|GetCurrentCameraPositionIndex) 1)))
              (Rendering|Components|TextRender|SetText _camera_currentnumber (Utilities|Text|ToText(Integer) (+ _output_get_2 1)))))
          (CallFunction|ChangeCamPosition (Variables|Default|GetCurrentCameraPositionIndex))
          (Default|CallCameraPositionChanged (Variables|Default|GetCurrentCameraPositionIndex)))))))

(event OnComponentBeginOverlap(Sphere)
  (params (OverlappedComponent :type Primitive%20Component%20Object%20Reference) (OtherActor :type Actor%20Object%20Reference) (OtherComp :type Primitive%20Component%20Object%20Reference) (OtherBodyIndex :type Integer) (bFromSweep :type Boolean) (SweepResult :type Hit%20Result%20Structure%20%28by%20ref%29))
  (bind _exitcylinder (Variables|Default|GetExitCylinder))
  (bind _exitcylinder_2 (Variables|Default|GetExitCylinder))
  (bind _numbercylinder (Variables|Default|GetNumberCylinder))
  (bind _numbercylinder_2 (Variables|Default|GetNumberCylinder))
  (bind _returnvalue (Transformation|GetRelativeTransform _numbercylinder_2))
  (bind _returnvalue_2 (Transformation|GetRelativeTransform _exitcylinder))
  (bind _returnvalue_3 (Transformation|GetRelativeTransform _exitcylinder_2))
  (bind _returnvalue_4 (Transformation|GetRelativeTransform _numbercylinder))
  (if (Actor|ActorHasTag OtherActor "Interactor")
    (if (Variables|Default|GetIsNotPaused)
      (if (not (Variables|Default|GetIsTransitioning))
        (Variables|Default|SetIsTransitioning true)
        (bind _newtrack_0 (Timeline|ExitTransitionTimeline PlayFromStart)
          (:Update
            (Transformation|SetRelativeLocation _exitcylinder_2 (Math|Vector|Lerp(Vector) (Math|Vector|MakeVector (.x (.location _returnvalue_3)) (.y (.location _returnvalue_3)) (.z (.location _returnvalue_3))) (Math|Vector|MakeVector (.x (.location _returnvalue_3)) (.y (.location _returnvalue_3)) -7e+01) _newtrack_0) false false)
            (Transformation|SetRelativeLocation _numbercylinder (Math|Vector|Lerp(Vector) (Math|Vector|MakeVector (.x (.location _returnvalue_4)) (.y (.location _returnvalue_4)) (.z (.location _returnvalue_4))) (Math|Vector|MakeVector (.x (.location _returnvalue_4)) -5.0 (.z (.location _returnvalue_4))) _newtrack_0) false false)
            (Rendering|Components|TextRender|SetText (Variables|Default|GetExit-Countdown) (Utilities|Text|ToText(String) ""))
            (Rendering|Material|SetScalarParameterValue (Variables|Default|GetDynamicExitMaterial) "Brightness" (Math|Float|Lerp 0.0 1.0 _newtrack_0) :!class /Script/Engine.MaterialInstanceDynamic)
            (Rendering|Material|SetScalarParameterValue (Variables|Default|GetDynamicExitTextMaterial) "Brightness" (Math|Float|Lerp 0.0 1.0 _newtrack_0) :!class /Script/Engine.MaterialInstanceDynamic))
          (:Finished
            (Variables|Default|SetIsNotPaused false)
            (bind _newtrack_0_2 (Timeline|ExitPauseTimeline PlayFromStart)
              (:Update
                (Rendering|Components|TextRender|SetText (Variables|Default|GetExit-Countdown) (Utilities|Text|ToText(String) (Class|KismetMathLibrary|Round64 _newtrack_0_2))))
              (:Finished
                (Variables|Default|SetIsNotPaused true)
                (Variables|Default|SetIsTransitioning true)
                (bind _newtrack_0_3 (Timeline|ExitResetTimeline PlayFromStart)
                  (:Update
                    (Transformation|SetRelativeLocation _exitcylinder (Math|Vector|Lerp(Vector) (Math|Vector|MakeVector (.x (.location _returnvalue_2)) (.y (.location _returnvalue_2)) (.z (.location _returnvalue_2))) (Math|Vector|MakeVector (.x (.location _returnvalue_2)) (.y (.location _returnvalue_2)) 0.0) _newtrack_0_3) false false)
                    (Transformation|SetRelativeLocation _numbercylinder_2 (Math|Vector|Lerp(Vector) (Math|Vector|MakeVector (.x (.location _returnvalue)) (.y (.location _returnvalue)) (.z (.location _returnvalue))) (Math|Vector|MakeVector (.x (.location _returnvalue)) 5.0 (.z (.location _returnvalue))) _newtrack_0_3) false false)
                    (Rendering|Material|SetScalarParameterValue (Variables|Default|GetDynamicExitMaterial) "Brightness" (Math|Float|Lerp 1.0 0.0 _newtrack_0_3) :!class /Script/Engine.MaterialInstanceDynamic)
                    (Rendering|Material|SetScalarParameterValue (Variables|Default|GetDynamicExitTextMaterial) "Brightness" (Math|Float|Lerp 1.0 0.0 _newtrack_0_3) :!class /Script/Engine.MaterialInstanceDynamic))
                  (:Finished
                    (Variables|Default|SetIsTransitioning false))))))))
      (else
        (CallFunction|ExitSession)
        (Default|CallExitSessionPressed)))))

(event Custom|SessionPrivate
  (Development|PrintString "Session Private"))

(event Custom|SessionPublic
  (Development|PrintString "Session Public"))

(event Custom|ChangeCamPosition
  (params (CamIndex :type Integer))
  (Development|PrintString (Utilities|String|Append "Switching to Camera Position " (Utilities|String|ToString(Integer) (+ CamIndex 1)))))

(event Custom|ExitSession
  (Development|PrintString "Exit Session"))

(fn ConstructionScript
  (bind _camera_currenttext (Variables|Default|GetCamera-CurrentText))
  (bind _togglemesh (Variables|Default|GetToggleMesh))
  (bind _session_toggletext (Variables|Default|GetSession-ToggleText))
  (bind _exit_titletext (Variables|Default|GetExit-TitleText))
  (bind _x1 (Variables|Default|GetX1))
  (bind _arrowmiddleright (Variables|Default|GetArrowMiddleRight))
  (bind _arrowmiddleleft (Variables|Default|GetArrowMiddleLeft))
  (Utilities|FlowControl|Sequence
    (:then_0
      (bind _returnvalue (Rendering|Material|CreateDynamicMaterialInstance _togglemesh 0 (Rendering|Material|GetMaterial _togglemesh 0) "ToggleMaterial" :!class /Script/Engine.PrimitiveComponent))
      (bind _output_get (Variables|Default|SetDynamicToggleMaterial _returnvalue))
      (Rendering|Material|SetMaterial _togglemesh 0 _output_get)
      (bind _returnvalue_2 (Rendering|Material|CreateDynamicMaterialInstance _session_toggletext 0 (Rendering|Material|GetMaterial _session_toggletext 0) "ToggleTextMaterial" :!class /Script/Engine.PrimitiveComponent))
      (bind _output_get_2 (Variables|Default|SetDynamicToggleTextMaterial _returnvalue_2))
      (Rendering|Material|SetMaterial _session_toggletext 0 _output_get_2))
    (:then_1
      (bind _returnvalue_3 (Rendering|Material|CreateDynamicMaterialInstance _x1 0 (Rendering|Material|GetMaterial _x1 0) "ExitMaterial" :!class /Script/Engine.PrimitiveComponent))
      (bind _output_get_3 (Variables|Default|SetDynamicExitMaterial _returnvalue_3))
      (Rendering|Material|SetMaterial _x1 0 _output_get_3)
      (bind _returnvalue_4 (Rendering|Material|CreateDynamicMaterialInstance _exit_titletext 0 (Rendering|Material|GetMaterial _exit_titletext 0) "ExitTextMaterial" :!class /Script/Engine.PrimitiveComponent))
      (bind _output_get_4 (Variables|Default|SetDynamicExitTextMaterial _returnvalue_4))
      (Rendering|Material|SetMaterial _exit_titletext 0 _output_get_4))
    (:then_2
      (bind _returnvalue_5 (Rendering|Material|CreateDynamicMaterialInstance _arrowmiddleright 0 (Rendering|Material|GetMaterial _arrowmiddleright 0) "ArrowRightMaterial" :!class /Script/Engine.PrimitiveComponent))
      (bind _output_get_5 (Variables|Default|SetDynamicRightArrowMaterial _returnvalue_5))
      (Rendering|Material|SetMaterial _arrowmiddleright 0 _output_get_5)
      (bind _returnvalue_6 (Rendering|Material|CreateDynamicMaterialInstance _camera_currenttext 0 (Rendering|Material|GetMaterial _camera_currenttext 0) "CurrentCameraTextMaterial" :!class /Script/Engine.PrimitiveComponent))
      (bind _output_get_6 (Variables|Default|SetDynamicCurrentCameraTextMaterial _returnvalue_6))
      (Rendering|Material|SetMaterial _camera_currenttext 0 _output_get_6))
    (:then_3
      (bind _returnvalue_7 (Rendering|Material|CreateDynamicMaterialInstance _arrowmiddleleft 0 (Rendering|Material|GetMaterial _arrowmiddleleft 0) "ArrowLeftMaterial" :!class /Script/Engine.PrimitiveComponent))
      (bind _output_get_7 (Variables|Default|SetDynamicLeftArrowMaterial _returnvalue_7))
      (Rendering|Material|SetMaterial _arrowmiddleleft 0 _output_get_7))))